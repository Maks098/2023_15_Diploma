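; BP_SaveGame is a save game object that stores and restores state for levers, checkpoints and boxes.
; It passes itself to savable objects through SaveDataMessage, and to a load requester through LoadDataMessage, leaving each object to handle its own data.
; LoadLastSave block-loads the keys of the three per-type save maps, casts each to its Blueprint class and calls its reload function.
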(fn `LoadDataForRequester`
  (params (Requester :type "Object Object Reference"))
  (message `/Game/Save/BPI_Savable.LoadData` Requester self)
  (return))

(fn `LoadLastSave`
  (`|ExecutionSequence`
    (:`then_0`
      (bind _keys (`BlueprintMapLibrary.Map_Keys` (`self.LeverSaveData`)))
      (for _array_element _keys
        (bind _returnvalue (`KismetSystemLibrary.LoadAsset_Blocking` _array_element))
        (bind _asbp_lever (cast `/Game/BlueprintClasses/Lever/BP_Lever` _returnvalue))
        (`/Game/Save/BPI_Savable.ReloadData` _asbp_lever)))
    (:`then_1`
      (bind _keys_2 (`BlueprintMapLibrary.Map_Keys` (`self.CheckpointSaveData`)))
      (for _array_element_2 _keys_2
        (bind _returnvalue_2 (`KismetSystemLibrary.LoadAsset_Blocking` _array_element_2))
        (bind _asbp_checkpoint (cast `/Game/BlueprintClasses/CheckPoint/BP_Checkpoint` _returnvalue_2))
        (message `/Game/Save/BPI_Savable.ReloadData` _asbp_checkpoint)))
    (:`then_2`
      (bind _keys_3 (`BlueprintMapLibrary.Map_Keys` (`self.BoxSaveData`)))
      (for _array_element_3 _keys_3
        (bind _returnvalue_3 (`KismetSystemLibrary.LoadAsset_Blocking` _array_element_3))
        (bind _asbp_old_box (cast `/Game/BlueprintClasses/BP_OldBox` _returnvalue_3))
        (message `/Game/Save/BPI_Savable.ReloadData` _asbp_old_box)))))

(fn `SaveAllData`
  (params (SavableObjects :type "Array of Object Object Reference"))
  (for _array_element SavableObjects
    (message `/Game/Save/BPI_Savable.SaveData` _array_element self))
  (return))