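; BP_InGameCamera is a level area that switches the player's view to one of its cameras while the third-person character is inside.
; Entering, or starting inside, enables input and applies the current camera, and keys 1 and 3 cycle through the camera array with wraparound.
; Each switch copies the camera's pitch and yaw to the character.
; Leaving disables input and briefly blocks re-entry through a short timer.
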(event `self.ReceiveBeginPlay`
  (bind _returnvalue (`GameplayStatics.GetPlayerController` 0))
  (bind _overlappingactors (`PrimitiveComponent.GetOverlappingActors` (`self.LevelArea`) "/Game/ThirdPerson/Blueprints/BP_ThirdPersonCharacter.BP_ThirdPersonCharacter_C"))
  (`KismetSystemLibrary.DelayUntilNextTick`)
  (if (> (`KismetArrayLibrary.Array_Length` _overlappingactors) 0)
    (bind _asbp_third_person_character (cast `/Game/ThirdPerson/Blueprints/BP_ThirdPersonCharacter` (`|GetArrayItem` _overlappingactors)))
    (set `self.ThirdPersonCharacter` _asbp_third_person_character)
    (if (`self.CanEnter`) :!label _label
      (`self.EnableInput` _returnvalue)
      (`self.SetCameraAndInputRotation` _returnvalue))))

(event `self.LevelArea.OnComponentBeginOverlap`
  (params (OverlappedComponent :type "PrimitiveComponent Object Reference") (OtherActor :type "Actor Object Reference") (OtherComp :type "PrimitiveComponent Object Reference") (OtherBodyIndex :type Integer) (bFromSweep :type Boolean) (SweepResult :type "HitResult Structure (by ref)"))
  (bind _asbp_third_person_character (cast `/Game/ThirdPerson/Blueprints/BP_ThirdPersonCharacter` OtherActor))
  (set `self.ThirdPersonCharacter` _asbp_third_person_character)
  (goto _label))

(event `self.LevelArea.OnComponentEndOverlap`
  (params (OverlappedComponent :type "PrimitiveComponent Object Reference") (OtherActor :type "Actor Object Reference") (OtherComp :type "PrimitiveComponent Object Reference") (OtherBodyIndex :type Integer))
  (cast `/Game/ThirdPerson/Blueprints/BP_ThirdPersonCharacter` OtherActor)
  (set `self.ThirdPersonCharacter` null)
  (`self.DisableInput` (`GameplayStatics.GetPlayerController` 0))
  (if (`KismetSystemLibrary.K2_IsValidTimerHandle` (`self.JustLeftHandle`))
    (`KismetSystemLibrary.K2_ClearAndInvalidateTimerHandle` (`self.JustLeftHandle`)))
  (set `self.CanEnter` false)
  (bind _returnvalue (`KismetSystemLibrary.K2_SetTimer` null "EnableEnter" 0.01))
  (set `self.JustLeftHandle` _returnvalue))

(event `Key|Three`
  (params (Key :type "Key Structure"))
  (:`Pressed`
    (bind _output_get (set `self.CurrentCamera` (+ (`self.CurrentCamera`) 1)))
    (if (>= _output_get (`KismetArrayLibrary.Array_Length` (`self.CameraActor`)))
      (set `self.CurrentCamera` 0))
    (`self.SetCameraAndInputRotation` (`GameplayStatics.GetPlayerController` 0) :!label _label_2)))

(event `Key|One`
  (params (Key :type "Key Structure"))
  (:`Pressed`
    (bind _output_get (set `self.CurrentCamera` (+ (`self.CurrentCamera`) -1)))
    (if (< _output_get 0)
      (set `self.CurrentCamera` (- (`KismetArrayLibrary.Array_Length` (`self.CameraActor`)) 1))
      (goto _label_2)
      (else
        (goto _label_2)))))

(fn `EnableEnter`
  (set `self.CanEnter` true)
  (`KismetSystemLibrary.K2_ClearAndInvalidateTimerHandle` (`self.JustLeftHandle`)))

(fn `SetCameraAndInputRotation`
  (params (PlayerController :type "PlayerController Object Reference"))
  (bind _output (`|GetArrayItem` (`self.CameraActor`) (`self.CurrentCamera`)))
  (bind (_returnvalue_roll _returnvalue_pitch _returnvalue_yaw) (`KismetMathLibrary.BreakRotator` (`self.K2_GetActorRotation` _output)))
  (`PlayerController.SetViewTargetWithBlend` PlayerController _output 0.0 "VTBlend_Linear" 0.0 false)
  (set `/Game/ThirdPerson/Blueprints/BP_ThirdPersonCharacter.CurrentCameraLocation` (`KismetMathLibrary.MakeRotator` 0.0 _returnvalue_pitch _returnvalue_yaw) (`self.ThirdPersonCharacter`)))

(fn `UserConstructionScript`)