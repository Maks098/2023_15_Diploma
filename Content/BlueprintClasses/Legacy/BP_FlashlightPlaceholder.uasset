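; Legacy placeholder flashlight actor that switches a child-actor quantum light component on or off.
; The construction script copies its state, ID, angle, line length, update frequency and trace-count settings to that child.
; On BeginPlay it enables player 0 input and applies the initial state.
; Pressing V toggles the state only while the flashlight is in hand, calling TurnOn or TurnOff on the child.
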(event `self.ReceiveBeginPlay`
  (`self.EnableInput` (`GameplayStatics.GetPlayerController` 0))
  (if (stale `Key|V` _output_get) :!label _label
    (`self.TurnOn`)
    (else
      (`self.TurnOff`))))

(event `Key|V`
  (params (Key :type "Key Structure"))
  (:`Pressed`
    (if (`self.InHand`)
      (bind _output_get (set `self.State` (not (`self.State`))))
      (goto _label))))

(event `TurnOn`
  (`|ExecutionSequence`
    (:`then_0`
      (bind _asbp_quantum_light_componenent (cast `/Game/BlueprintClasses/QuantumComponents/QuantumLight/BP_QuantumLightComponenent` (`ChildActorComponent.ChildActor` (`self.BP_QuantumLightComponenent`)) :!label _label_2)))
    (:`then_1`
      (`/Game/BlueprintClasses/QuantumComponents/QuantumLight/BP_QuantumLightComponenent.TurnOn` _asbp_quantum_light_componenent))))

(event `TurnOff`
  (`|ExecutionSequence`
    (:`then_0`
      (goto _label_2))
    (:`then_1`
      (`/Game/BlueprintClasses/QuantumComponents/QuantumLight/BP_QuantumLightComponenent.TurnOff` (stale `TurnOn` _asbp_quantum_light_componenent)))))

(fn `UserConstructionScript`
  (bind _asbp_quantum_light_componenent (cast `/Game/BlueprintClasses/QuantumComponents/QuantumLight/BP_QuantumLightComponenent` (`ChildActorComponent.ChildActor` (`self.BP_QuantumLightComponenent`))))
  (set `/Game/BlueprintClasses/QuantumComponents/QuantumLight/BP_QuantumLightComponenent.AngleRange` (`self.Angle Range`) _asbp_quantum_light_componenent)
  (set `/Game/BlueprintClasses/QuantumComponents/QuantumLight/BP_QuantumLightComponenent.IdLightSource` (`self.Id Light Source`) _asbp_quantum_light_componenent)
  (set `/Game/BlueprintClasses/QuantumComponents/QuantumLight/BP_QuantumLightComponenent.State` (`self.State`) _asbp_quantum_light_componenent)
  (set `/Game/BlueprintClasses/QuantumComponents/QuantumLight/BP_QuantumLightComponenent.LineLength` (`self.Line Length`) _asbp_quantum_light_componenent)
  (set `/Game/BlueprintClasses/QuantumComponents/QuantumLight/BP_QuantumLightComponenent.UpdateFrequency` (`self.Update Frequency`) _asbp_quantum_light_componenent)
  (set `/Game/BlueprintClasses/QuantumComponents/QuantumLight/BP_QuantumLightComponenent.NumOfTracesPitch` (`self.Num Of Traces Pitch`) _asbp_quantum_light_componenent)
  (set `/Game/BlueprintClasses/QuantumComponents/QuantumLight/BP_QuantumLightComponenent.NumOfTracesYaw` (`self.Num Of Traces Yaw`) _asbp_quantum_light_componenent))