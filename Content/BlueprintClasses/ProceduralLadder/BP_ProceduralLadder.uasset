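; Climbable ladder actor that builds itself procedurally from a height, with instanced rungs, optional screws at intervals and optional curved pole ends.
; The construction script also sizes an interaction box whose overlap enables input and caches the third-person character.
; E attaches or detaches by toggling flying and falling movement, and Space jumps off.
; Holding W or S runs looping timers that nudge the character vertically between the pole ends.
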(event `Key|SpaceBar`
  (params (Key :type "Key Structure"))
  (bind _characterreference (`self.CharacterReference`))
  (:`Pressed`
    (if (`/Game/ThirdPerson/Blueprints/BP_ThirdPersonCharacter.IsInLadder?` _characterreference)
      (`self.Detach Player From Ladder`)
      (`Character.LaunchCharacter` _characterreference (`KismetMathLibrary.MakeVector` 0.0 0.0 (`CharacterMovementComponent.JumpZVelocity` (`Character.CharacterMovement` _characterreference))) false false))))

(event `Key|W`
  (params (Key :type "Key Structure"))
  (bind _characterreference (`self.CharacterReference`))
  (:`Pressed`
    (if (`/Game/ThirdPerson/Blueprints/BP_ThirdPersonCharacter.IsInLadder?` _characterreference)
      (set `/Game/ThirdPerson/Blueprints/BP_ThirdPersonCharacter.isClimbingUpLadder?` true _characterreference)
      (bind _returnvalue (`KismetSystemLibrary.K2_SetTimerDelegate` (delegate `ClimbUp`) 0.01 true))
      (set `self.ClimbUpHandle` _returnvalue)))
  (:`Released`
    (`KismetSystemLibrary.K2_ClearAndInvalidateTimerHandle` (`self.ClimbUpHandle`))
    (set `/Game/ThirdPerson/Blueprints/BP_ThirdPersonCharacter.isClimbingUpLadder?` false _characterreference)))

(event `ClimbUp`
  (`self.Climbing Up`))

(event `Key|S`
  (params (Key :type "Key Structure"))
  (bind _characterreference (`self.CharacterReference`))
  (:`Pressed`
    (if (`/Game/ThirdPerson/Blueprints/BP_ThirdPersonCharacter.IsInLadder?` _characterreference)
      (set `/Game/ThirdPerson/Blueprints/BP_ThirdPersonCharacter.isClimbingDownLadder?` true _characterreference)
      (bind _returnvalue (`KismetSystemLibrary.K2_SetTimerDelegate` (delegate `ClimbDown`) 0.01 true))
      (set `self.ClimbDownHandle` _returnvalue)))
  (:`Released`
    (`KismetSystemLibrary.K2_ClearAndInvalidateTimerHandle` (`self.ClimbDownHandle`))
    (set `/Game/ThirdPerson/Blueprints/BP_ThirdPersonCharacter.isClimbingDownLadder?` false _characterreference)))

(event `ClimbDown`
  (`self.Climbing Down`))

(event `Key|E`
  (params (Key :type "Key Structure"))
  (:`Pressed`
    (if (`/Game/ThirdPerson/Blueprints/BP_ThirdPersonCharacter.IsInLadder?` (`self.CharacterReference`))
      (`self.Detach Player From Ladder`)
      (else
        (`self.Attach Player To Ladder`)))))

(event `self.InteractionBox.OnComponentBeginOverlap`
  (params (OverlappedComponent :type "PrimitiveComponent Object Reference") (OtherActor :type "Actor Object Reference") (OtherComp :type "PrimitiveComponent Object Reference") (OtherBodyIndex :type Integer) (bFromSweep :type Boolean) (SweepResult :type "HitResult Structure (by ref)"))
  (bind _asbp_third_person_character (cast `/Game/ThirdPerson/Blueprints/BP_ThirdPersonCharacter` OtherActor))
  (set `self.CharacterReference` _asbp_third_person_character)
  (`self.EnableInput` (`GameplayStatics.GetPlayerController` 0)))

(event `self.InteractionBox.OnComponentEndOverlap`
  (params (OverlappedComponent :type "PrimitiveComponent Object Reference") (OtherActor :type "Actor Object Reference") (OtherComp :type "PrimitiveComponent Object Reference") (OtherBodyIndex :type Integer))
  (cast `/Game/ThirdPerson/Blueprints/BP_ThirdPersonCharacter` OtherActor)
  (`self.DisableInput` (`GameplayStatics.GetPlayerController` 0))
  (set `self.CharacterReference` null))

(fn `Attach Player To Ladder`
  (bind (_returnvalue_x _returnvalue_y) (`KismetMathLibrary.BreakVector` (`SceneComponent.K2_GetComponentLocation` (`self.ClimbingPosition`))))
  (bind _capsulecomponent (`Character.CapsuleComponent` (`self.CharacterReference`)))
  (bind (_returnvalue_x_2 _returnvalue_y_2 _returnvalue_z) (`KismetMathLibrary.BreakVector` (`SceneComponent.K2_GetComponentLocation` _capsulecomponent)))
  (`SceneComponent.K2_SetWorldLocation` _capsulecomponent (`KismetMathLibrary.MakeVector` _returnvalue_x _returnvalue_y _returnvalue_z) false false)
  (`SceneComponent.K2_SetWorldRotation` _capsulecomponent (`SceneComponent.K2_GetComponentRotation` (`self.InteractionBox`)) false false)
  (`self.Set Player Climbing State`)
  (set `/Game/ThirdPerson/Blueprints/BP_ThirdPersonCharacter.IsInLadder?` true (`self.CharacterReference`)))

(fn `Detach Player From Ladder`
  (bind _characterreference (`self.CharacterReference`))
  (bind _climbuphandle (`self.ClimbUpHandle`))
  (bind _climbdownhandle (`self.ClimbDownHandle`))
  (`self.Set Player Normal State`)
  (set `/Game/ThirdPerson/Blueprints/BP_ThirdPersonCharacter.IsInLadder?` false (`self.CharacterReference`))
  (`|ExecutionSequence`
    (:`then_0`
      (if (`KismetSystemLibrary.K2_IsTimerActiveHandle` _climbuphandle)
        (`KismetSystemLibrary.K2_ClearAndInvalidateTimerHandle` _climbuphandle)
        (set `/Game/ThirdPerson/Blueprints/BP_ThirdPersonCharacter.isClimbingUpLadder?` false _characterreference)))
    (:`then_1`
      (if (`KismetSystemLibrary.K2_IsTimerActiveHandle` _climbdownhandle)
        (`KismetSystemLibrary.K2_ClearAndInvalidateTimerHandle` _climbdownhandle)
        (set `/Game/ThirdPerson/Blueprints/BP_ThirdPersonCharacter.isClimbingDownLadder?` false _characterreference)))))

(fn `Set Ladder End Pieces`
  (bind _returnvalue (* (`self.Ladder Height`) 100.0))
  (bind _returnvalue_2 (select `/Game/BlueprintClasses/ProceduralLadder/E_LadderEndTypes` (`self.End Type`) :`NewEnumerator1` "/Game/StarterContent/Shapes/Shape_Pipe_180.Shape_Pipe_180" :!type "StaticMesh Object Reference"))
  (`SceneComponent.K2_SetRelativeLocation` (`self.LeftPoleEnd`) (`KismetMathLibrary.MakeVector` 11.182681 -34.793804 _returnvalue) false false)
  (`SceneComponent.K2_SetRelativeLocation` (`self.RightPoleEnd`) (`KismetMathLibrary.MakeVector` 11.182681 25.206196 _returnvalue) false false)
  (`StaticMeshComponent.SetStaticMesh` (`self.LeftPoleEnd`) _returnvalue_2)
  (`StaticMeshComponent.SetStaticMesh` (`self.RightPoleEnd`) _returnvalue_2))

(fn `Set Player Climbing State`
  (bind _characterreference (`self.CharacterReference`))
  (bind _charactermovement (`Character.CharacterMovement` _characterreference))
  (set `/Game/ThirdPerson/Blueprints/BP_ThirdPersonCharacter.CanMove?` false _characterreference)
  (set `CharacterMovementComponent.GravityScale` 0.0 _charactermovement)
  (`CharacterMovementComponent.SetMovementMode` _charactermovement "MOVE_Flying" 0)
  (set `CharacterMovementComponent.BrakingDecelerationFlying` 4000.0 _charactermovement)
  (set `CharacterMovementComponent.MaxAcceleration` 1.0 _charactermovement))

(fn `Set Player Normal State`
  (bind _characterreference (`self.CharacterReference`))
  (bind _charactermovement (`Character.CharacterMovement` _characterreference))
  (set `/Game/ThirdPerson/Blueprints/BP_ThirdPersonCharacter.CanMove?` true _characterreference)
  (set `CharacterMovementComponent.GravityScale` 1.75 _charactermovement)
  (`CharacterMovementComponent.SetMovementMode` _charactermovement "MOVE_Falling" 0)
  (set `CharacterMovementComponent.BrakingDecelerationFlying` 0.0 _charactermovement)
  (set `CharacterMovementComponent.MaxAcceleration` 1500.0 _charactermovement))

(fn `UserConstructionScript`
  (bind (_relativelocation_x _relativelocation_y _relativelocation_z) (`KismetMathLibrary.BreakVector` (`SceneComponent.RelativeLocation` (`self.LeftPoleEnd`))))
  (`SceneComponent.SetRelativeScale3D` (`self.InteractionBox`) (`KismetMathLibrary.MakeVector` 1.0 1.0 (* (`self.Ladder Height`) 1.6)))
  (`SceneComponent.SetRelativeScale3D` (`self.LadderLeftPole`) (`KismetMathLibrary.MakeVector` 0.1 0.1 (`self.Ladder Height`)))
  (`SceneComponent.SetRelativeScale3D` (`self.LadderRightPole`) (`KismetMathLibrary.MakeVector` 0.1 0.1 (`self.Ladder Height`)))
  (while (< (`self.Compare Height`) (* (`self.Ladder Height`) 100.0))
    (`self.Add bars and screws`))
  (`self.Set Ladder End Pieces`)
  (`SceneComponent.K2_SetRelativeLocation` (`self.InteractionBox`) (`KismetMathLibrary.MakeVector` -30.0 0.0 (/ _relativelocation_z 2.0)) false false))