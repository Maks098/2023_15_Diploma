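; Pullable box that the player can grab with the left mouse button and move around while standing in its trigger.
; Overlap stores the third-person character and enables input; releasing the button or leaving the trigger releases the box.
; Grabbing slows the character and stops it orienting to movement.
; While grabbed, move input is remapped by the character mesh's rounded right vector, then interpolates the box along its own axes, tuned to walk speed.
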(event `Key|LeftMouseButton`
  (params (Key :type "Key Structure"))
  (:`Pressed`
    (if (`self.isPlayerOverlapping?`)
      (`self.Grab Box`)))
  (:`Released`
    (`self.Release Box`)))

(event `self.Box.OnComponentBeginOverlap`
  (params (OverlappedComponent :type "PrimitiveComponent Object Reference") (OtherActor :type "Actor Object Reference") (OtherComp :type "PrimitiveComponent Object Reference") (OtherBodyIndex :type Integer) (bFromSweep :type Boolean) (SweepResult :type "HitResult Structure (by ref)"))
  (bind _asbp_third_person_character (cast `/Game/ThirdPerson/Blueprints/BP_ThirdPersonCharacter` OtherActor))
  (set `self.isPlayerOverlapping?` true)
  (set `self.CharacterReference` _asbp_third_person_character)
  (`self.EnableInput` (`GameplayStatics.GetPlayerController` 0)))

(event `self.Box.OnComponentEndOverlap`
  (params (OverlappedComponent :type "PrimitiveComponent Object Reference") (OtherActor :type "Actor Object Reference") (OtherComp :type "PrimitiveComponent Object Reference") (OtherBodyIndex :type Integer))
  (cast `/Game/ThirdPerson/Blueprints/BP_ThirdPersonCharacter` OtherActor)
  (set `self.isPlayerOverlapping?` false)
  (`self.Release Box`)
  (`self.DisableInput` (`GameplayStatics.GetPlayerController` 0)))

(event `EnhancedInput|/Game/ThirdPerson/Input/Actions/IA_Move`
  (params (ActionValue :type "Vector2D Structure") (ElapsedSeconds :type "Float (double-precision)") (TriggeredSeconds :type "Float (double-precision)") (InputAction :type "InputAction Object Reference" :default "/Game/ThirdPerson/Input/Actions/IA_Move.IA_Move"))
  (bind _returnvalue (`GameplayStatics.GetWorldDeltaSeconds`))
  (bind _staticmesh (`self.StaticMesh`))
  (bind _returnvalue_2 (`SceneComponent.K2_GetComponentLocation` _staticmesh))
  (bind _returnvalue_3 (* (`self.Action Value X`) 15.0))
  (bind _returnvalue_4 (* (`self.Action Value Y`) 15.0))
  (bind (_returnvalue_x _returnvalue_y) (`KismetMathLibrary.BreakVector` (`SceneComponent.GetRightVector` (`Character.Mesh` (`self.CharacterReference`)))))
  (bind _returnvalue_5 (`KismetMathLibrary.Round` _returnvalue_x))
  (bind _returnvalue_6 (`KismetMathLibrary.Round` _returnvalue_y))
  (:`Triggered`
    (if (!= _returnvalue_5 0)
      (set `self.Action Value X` (* ActionValue_X _returnvalue_5))
      (set `self.Action Value Y` (* ActionValue_Y _returnvalue_5))
      (else
        (set `self.Action Value X` (* ActionValue_Y _returnvalue_6))
        (set `self.Action Value Y` (* ActionValue_X (* _returnvalue_6 -1)))))
    (if (`self.isPlayerGrabbing?`)
      (`|ExecutionSequence`
        (:`then_0`
          (if (!= _returnvalue_3 0.0)
            (`SceneComponent.K2_SetWorldLocation` (`self.StaticMesh`) (`KismetMathLibrary.VInterpTo` _returnvalue_2 (+ _returnvalue_2 (* (`SceneComponent.GetRightVector` _staticmesh) _returnvalue_3)) _returnvalue 4.0) false false)))
        (:`then_1`
          (if (!= _returnvalue_4 0.0)
            (`SceneComponent.K2_SetWorldLocation` (`self.StaticMesh`) (`KismetMathLibrary.VInterpTo` _returnvalue_2 (+ (* (`SceneComponent.GetForwardVector` (`self.StaticMesh`)) _returnvalue_4) _returnvalue_2) _returnvalue 4.0) false false)))))))

(fn `Grab Box`
  (bind _charactermovement (`Character.CharacterMovement` (`self.CharacterReference`)))
  (set `CharacterMovementComponent.MaxWalkSpeed` (- (`CharacterMovementComponent.MaxWalkSpeed` _charactermovement) 440.0) _charactermovement)
  (`PrimitiveComponent.SetSimulatePhysics` (`self.StaticMesh`) true)
  (set `CharacterMovementComponent.bOrientRotationToMovement` false (`Character.CharacterMovement` (`self.CharacterReference`)))
  (set `self.isPlayerGrabbing?` true))

(fn `Release Box`
  (set `CharacterMovementComponent.MaxWalkSpeed` 500.0 (`Character.CharacterMovement` (`self.CharacterReference`)))
  (`PrimitiveComponent.SetSimulatePhysics` (`self.StaticMesh`) true)
  (set `CharacterMovementComponent.bOrientRotationToMovement` true (`Character.CharacterMovement` (`self.CharacterReference`)))
  (set `self.isPlayerGrabbing?` false))

(fn `UserConstructionScript`)