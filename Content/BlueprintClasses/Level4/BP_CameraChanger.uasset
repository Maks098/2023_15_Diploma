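; BP_CameraChanger plays a timed camera cutaway in Level 4 while an interactable switches on or off.
; Turnon and TurnOff each lock player movement, switch view to CameraToChange, then toggle the Interactable after configurable delays.
; Both paths share a tail that restores movement, then the player's old camera.
; Two DoOnce gates reset each other so the events alternate without repeating.
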(event `/Game/BlueprintClasses/OnOffInterface.TurnOn`
  (bind _player (`self.Player`))
  (`/Engine/EditorBlueprintResources/StandardMacros.DoOnce` false :!label _label
    (:`Completed`
      (`|ExecutionSequence`
        (:`then_0`
          (`KismetSystemLibrary.Delay` (`self.DurationOfFirstDelay`))
          (`/Game/ThirdPerson/Blueprints/BP_ThirdPersonCharacter.TurnOffMovement` (`self.Player`))
          (`PlayerController.SetViewTargetWithBlend` (`GameplayStatics.GetPlayerController` 0) (`self.CameraToChange`) 0.0 "VTBlend_Linear" 0.0 false)
          (`KismetSystemLibrary.Delay` (`self.DurationOfSecondDelay`))
          (`/Game/BlueprintClasses/OnOffInterface.TurnOn` (`self.Interactable`))
          (`KismetSystemLibrary.Delay` 1.0)
          (`/Game/ThirdPerson/Blueprints/BP_ThirdPersonCharacter.TurnOnMovement` _player :!label _label_2)
          (`KismetSystemLibrary.Delay` (`self.DurationOfThirdDelay`))
          (`/Game/ThirdPerson/Blueprints/BP_ThirdPersonCharacter.SetOldCamera` _player))
        (:`then_1`
          (goto _label_3 :!via `Reset`))))))

(event `/Game/BlueprintClasses/OnOffInterface.TurnOff`
  (`/Engine/EditorBlueprintResources/StandardMacros.DoOnce` true :!label _label_3
    (:`Completed`
      (`|ExecutionSequence`
        (:`then_0`
          (`KismetSystemLibrary.Delay` (`self.DurationOfFirstDelay`))
          (`/Game/ThirdPerson/Blueprints/BP_ThirdPersonCharacter.TurnOffMovement` (`self.Player`))
          (`PlayerController.SetViewTargetWithBlend` (`GameplayStatics.GetPlayerController` 0) (`self.CameraToChange`) 0.0 "VTBlend_Linear" 0.0 false)
          (`KismetSystemLibrary.Delay` (`self.DurationOfSecondDelay`))
          (`/Game/BlueprintClasses/OnOffInterface.TurnOff` (`self.Interactable`))
          (goto _label_2))
        (:`then_1`
          (goto _label :!via `Reset`))))))

(event `self.ReceiveBeginPlay`
  (bind _returnvalue (`GameplayStatics.GetActorOfClass` "/Game/ThirdPerson/Blueprints/BP_ThirdPersonCharacter.BP_ThirdPersonCharacter_C"))
  (set `self.Player` _returnvalue))

(fn `UserConstructionScript`)