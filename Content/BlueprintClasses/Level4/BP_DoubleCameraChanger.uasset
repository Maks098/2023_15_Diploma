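; BP_DoubleCameraChanger is a Level 4 actor that plays timed camera cuts around switching an Interactable on or off.
; Turnon locks player movement, shows two cameras in sequence, then activates the Interactable.
; TurnOff waits first, then locks movement, shows only the second camera and deactivates it.
; Both paths restore movement, then return to a set camera after a final delay, using the third-person character found at BeginPlay.
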(event `self.TurnOn`
  (bind _returnvalue (`GameplayStatics.GetPlayerController` 0))
  (`/Game/ThirdPerson/Blueprints/BP_ThirdPersonCharacter.TurnOffMovement` (`self.Player`))
  (`PlayerController.SetViewTargetWithBlend` _returnvalue (`self.FirstCameraToChange`) 0.0 "VTBlend_Linear" 0.0 false)
  (`KismetSystemLibrary.Delay` (`self.DurationOfFirstDelay`))
  (`PlayerController.SetViewTargetWithBlend` _returnvalue (`self.SecondCameraToChange`) 0.0 "VTBlend_Linear" 0.0 false)
  (`KismetSystemLibrary.Delay` (`self.DurationOfSecondDelay`))
  (`/Game/BlueprintClasses/OnOffInterface.TurnOn` (`self.Interactable`))
  (`/Game/ThirdPerson/Blueprints/BP_ThirdPersonCharacter.TurnOnMovement` (`self.Player`) :!label _label)
  (`KismetSystemLibrary.Delay` (`self.DurationOfThirdDelay`))
  (`PlayerController.SetViewTargetWithBlend` (`GameplayStatics.GetPlayerController` 0) (`self.CameraToGoBackTo`) 0.0 "VTBlend_Linear" 0.0 false))

(event `self.TurnOff`
  (`KismetSystemLibrary.Delay` (`self.DurationOfFirstDelay`))
  (`/Game/ThirdPerson/Blueprints/BP_ThirdPersonCharacter.TurnOffMovement` (`self.Player`))
  (`PlayerController.SetViewTargetWithBlend` (`GameplayStatics.GetPlayerController` 0) (`self.SecondCameraToChange`) 0.0 "VTBlend_Linear" 0.0 false)
  (`KismetSystemLibrary.Delay` (`self.DurationOfSecondDelay`))
  (`/Game/BlueprintClasses/OnOffInterface.TurnOff` (`self.Interactable`))
  (goto _label))

(event `self.ReceiveBeginPlay`
  (bind _returnvalue (`GameplayStatics.GetActorOfClass` "/Game/ThirdPerson/Blueprints/BP_ThirdPersonCharacter.BP_ThirdPersonCharacter_C"))
  (set `self.Player` _returnvalue))

(fn `UserConstructionScript`)