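; Scripted camera sequence actor that, on Turnon, shows two cameras in succession and then returns the player to their previous camera.
; It disables player movement, switches views with timed delays, then turns on a linked Interactable.
; Movement resumes before a final delay and the call to the character's SetOldCamera.
; TurnOff is empty; its apparent reverse sequence is left disconnected.
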(event `self.TurnOn`
  (bind _returnvalue (`GameplayStatics.GetPlayerController` 0))
  (bind _player (`self.Player`))
  (`/Game/ThirdPerson/Blueprints/BP_ThirdPersonCharacter.TurnOffMovement` (`self.Player`))
  (`KismetSystemLibrary.PrintString` "Hello")
  (`PlayerController.SetViewTargetWithBlend` _returnvalue (`self.FirstCameraToChange`) 0.0 "VTBlend_Linear" 0.0 false)
  (`KismetSystemLibrary.Delay` (`self.DurationOfFirstDelay`))
  (`PlayerController.SetViewTargetWithBlend` _returnvalue (`self.SecondCameraToChange`) 0.0 "VTBlend_Linear" 0.0 false)
  (`KismetSystemLibrary.Delay` (`self.DurationOfSecondDelay`))
  (`/Game/BlueprintClasses/OnOffInterface.TurnOn` (`self.Interactable`))
  (`/Game/ThirdPerson/Blueprints/BP_ThirdPersonCharacter.TurnOnMovement` _player)
  (`KismetSystemLibrary.Delay` (`self.DurationOfThirdDelay`))
  (`/Game/ThirdPerson/Blueprints/BP_ThirdPersonCharacter.SetOldCamera` _player))

(event `self.TurnOff`)

(event `self.ReceiveBeginPlay`
  (bind _returnvalue (`GameplayStatics.GetActorOfClass` "/Game/ThirdPerson/Blueprints/BP_ThirdPersonCharacter.BP_ThirdPersonCharacter_C"))
  (set `self.Player` _returnvalue))

(fn `UserConstructionScript`)