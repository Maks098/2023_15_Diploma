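; Quantum light actor that casts a spotlight cone bounded by side panels and notifies QuantumLightDetectors it reaches.
; A looping timer sweeps yaw and pitch multi-line traces clipped to the cone, calling detectors until another quantum light blocks the trace.
; Edge hits from the first sweep resize the left and right panels to shape light subtraction.
; TurnOn/TurnOff toggle the timer, visibility, panel collision and shadows.
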(event `self.ReceiveBeginPlay`
  (`self.ScaleLight`)
  (`self.EnableInput` (`GameplayStatics.GetPlayerController` 0))
  (bind _returnvalue (`KismetSystemLibrary.K2_SetTimer` null "Create 3D Cone" (/ 1.0 (`self.UpdateFrequency`)) true))
  (set `self.FrequencyTimerHandle` _returnvalue))

(event `TurnOff`
  (`KismetSystemLibrary.K2_PauseTimerHandle` (`self.FrequencyTimerHandle`))
  (set `self.State` false)
  (`SceneComponent.SetVisibility` (`self.R Outside Panel`) false true)
  (`SceneComponent.SetVisibility` (`self.L Outside Panel`) false true)
  (`SceneComponent.SetVisibility` (`self.R Inside Panel`) false true)
  (`SceneComponent.SetVisibility` (`self.L Inside Panel`) false true)
  (`SceneComponent.SetVisibility` (`self.SpotLight`) false true)
  (`PrimitiveComponent.SetCollisionEnabled` (`self.R Outside Panel`) "NoCollision")
  (`PrimitiveComponent.SetCollisionEnabled` (`self.R Inside Panel`) "NoCollision")
  (`PrimitiveComponent.SetCollisionEnabled` (`self.L Outside Panel`) "NoCollision")
  (`PrimitiveComponent.SetCollisionEnabled` (`self.L Inside Panel`) "NoCollision")
  (`PrimitiveComponent.SetCastShadow` (`self.R Outside Panel`) false)
  (`PrimitiveComponent.SetCastShadow` (`self.R Inside Panel`) false)
  (`PrimitiveComponent.SetCastShadow` (`self.L Outside Panel`) false)
  (`PrimitiveComponent.SetCastShadow` (`self.L Inside Panel`) false))

(event `TurnOn`
  (`KismetSystemLibrary.K2_UnPauseTimerHandle` (`self.FrequencyTimerHandle`))
  (set `self.State` true)
  (`SceneComponent.SetVisibility` (`self.R Outside Panel`) true true)
  (`SceneComponent.SetVisibility` (`self.L Outside Panel`) true true)
  (`SceneComponent.SetVisibility` (`self.R Inside Panel`) true true)
  (`SceneComponent.SetVisibility` (`self.L Inside Panel`) true true)
  (`SceneComponent.SetVisibility` (`self.SpotLight`) true true)
  (`PrimitiveComponent.SetCollisionEnabled` (`self.R Outside Panel`) "QueryOnly")
  (`PrimitiveComponent.SetCollisionEnabled` (`self.R Inside Panel`) "QueryOnly")
  (`PrimitiveComponent.SetCollisionEnabled` (`self.L Outside Panel`) "QueryOnly")
  (`PrimitiveComponent.SetCollisionEnabled` (`self.L Inside Panel`) "QueryOnly")
  (`PrimitiveComponent.SetCastShadow` (`self.R Outside Panel`) true)
  (`PrimitiveComponent.SetCastShadow` (`self.R Inside Panel`) true)
  (`PrimitiveComponent.SetCastShadow` (`self.L Outside Panel`) true)
  (`PrimitiveComponent.SetCastShadow` (`self.L Inside Panel`) true))

(fn `CalculateAngleBetweenTwoVectors`
  (params (`Vector A` :type "Vector Structure") (`Vector B` :type "Vector Structure"))
  (returns (Angle :type "Float (double-precision)"))
  (return (`KismetMathLibrary.DegAcos` (/ (`KismetMathLibrary.Dot_VectorVector` `Vector A` `Vector B`) (* (`KismetMathLibrary.VSize` `Vector A`) (`KismetMathLibrary.VSize` `Vector B`))))))

(fn `Create 2D Cone`
  (params (`Y (Pitch)` :type "Float (single-precision)") (IsFIrtstIn :type Boolean))
  (locals (Index :type Integer) (UpOrDown :type "Float (double-precision)" :default -1.0) (Pitch :type "Float (single-precision)"))
  (bind _returnvalue (`self.K2_GetActorLocation`))
  (bind _index (`local.Index`))
  (bind _isfirtstin (`local.IsFIrtstIn`))
  (set `local.Pitch` `Y (Pitch)`)
  (if (== (mod (`KismetMathLibrary.FTrunc` `Y (Pitch)`) 2) 0)
    (set `local.Pitch` (/ (`local.Pitch`) 2.0))
    (else
      (set `local.Pitch` (/ (+ (`local.Pitch`) 1.0) -2.0))))
  (for _index_2 (range (+ (`self.NumOfTracesYaw`) 1))
    (set `local.Index` _index_2)
    (bind _returnvalue_2 (`KismetMathLibrary.RotateAngleAxis` (`KismetMathLibrary.GreaterGreater_VectorRotator` (`KismetMathLibrary.CreateVectorFromYawPitch` (* (`KismetMathLibrary.Conv_IntToDouble` (`self.AngleRange`)) -0.5) (* (/ (`KismetMathLibrary.Conv_IntToDouble` (`self.AngleRange`)) (`KismetMathLibrary.Conv_IntToDouble` (`self.NumOfTracesPitch`))) (`local.Pitch`))) (`self.K2_GetActorRotation`)) (* (`KismetMathLibrary.Conv_IntToDouble` _index_2) (/ (`KismetMathLibrary.Conv_IntToDouble` (`self.AngleRange`)) (`KismetMathLibrary.Conv_IntToDouble` (`self.NumOfTracesYaw`)))) (0.0 0.0 1.0)))
    ;[1 1 1] Check if Trace is in cone.
    (bind _angle (`self.CalculateAngleBetweenTwoVectors` (`self.GetActorForwardVector`) _returnvalue_2))
    (if (<= _angle (/ (+ (`KismetMathLibrary.Conv_IntToDouble` (`self.AngleRange`)) 0.01) 2.0))
      (bind _outhits (`KismetSystemLibrary.LineTraceMulti` :`Start` _returnvalue :`End` (+ _returnvalue (* (`self.LineLength`) _returnvalue_2)) :`TraceChannel` "TraceTypeQuery3" :`DrawDebugType` (`self.Draw Debug Type`) :`DrawTime` (/ 1.0 (`self.UpdateFrequency`))))
      (`self.Process Hits in Once Trace` _outhits (and (== _index 0) _isfirtstin) (and _isfirtstin (== _index (`self.NumOfTracesYaw`)))))))

(fn `Create 3D Cone`
  (locals (LeftLength :type "Float (double-precision)") (RightLength :type "Float (double-precision)") (LeftLines :type "Array of Float (double-precision)") (RightLines :type "Array of Float (double-precision)"))
  (bind _linelength (`self.LineLength`))
  (bind _leftlines (`local.LeftLines`))
  (bind _rightlines (`local.RightLines`))
  (bind _leftlines_2 (`local.LeftLines`))
  (bind _rightlines_2 (`local.RightLines`))
  (bind (_firsthitidlight _hitpanelsleft _hitpanelsright) (break `/Game/DataTypes/Structs/DataForPanelsInTrace` (`self.DataForPanels`)))
  (set `self.DataForPanels` (make `/Game/DataTypes/Structs/DataForPanelsInTrace` -1))
  (for _index (range (+ (`self.NumOfTracesPitch`) 1))
    (bind _returnvalue (== _index 0))
    (`self.Create 2D Cone` (`KismetMathLibrary.Conv_IntToDouble` _index) _returnvalue)
    (if _returnvalue
      (if (and (== _firsthitidlight -1) (== (`KismetArrayLibrary.Array_LastIndex` _hitpanelsleft) -1) (== (`KismetArrayLibrary.Array_LastIndex` _hitpanelsright) -1))
        (`self.ScalePanelsToUnits` _linelength _linelength)
        (else
          (set `local.LeftLines` _hitpanelsleft)
          (set `local.RightLines` _hitpanelsright)
          (`|ExecutionSequence`
            (:`then_0`
              ;[1 1 1] Set length to full if nothing hit.
              (if (== (`KismetArrayLibrary.Array_LastIndex` (`local.LeftLines`)) -1)
                (set `local.LeftLength` (`self.LineLength`))
                (else
                  (set `local.LeftLength` (`|GetArrayItem` _leftlines (`KismetArrayLibrary.Array_LastIndex` _leftlines)))))
              (if (== (`KismetArrayLibrary.Array_LastIndex` (`local.RightLines`)) -1)
                (set `local.RightLength` (`self.LineLength`))
                (else
                  (set `local.RightLength` (`|GetArrayItem` _rightlines (`KismetArrayLibrary.Array_LastIndex` _rightlines))))))
            (:`then_1`
              ;[1 1 1] Get the right shape for light subtraction.
              (if (and (> (`KismetArrayLibrary.Array_Length` (`local.LeftLines`)) 2) (> (`KismetArrayLibrary.Array_Length` (`local.RightLines`)) 2))
                (if (< (- (`|GetArrayItem` _leftlines_2 (`KismetArrayLibrary.Array_LastIndex` _leftlines_2)) (`|GetArrayItem` _leftlines_2)) (- (`|GetArrayItem` _rightlines_2 (`KismetArrayLibrary.Array_LastIndex` _rightlines_2)) (`|GetArrayItem` _rightlines_2)))
                  (set `local.RightLength` (`|GetArrayItem` (`local.RightLines`)))
                  (else
                    (set `local.LeftLength` (`|GetArrayItem` (`local.LeftLines`)))))))
            (:`then_2`
              (`self.ScalePanelsToUnits` (`local.LeftLength`) (`local.RightLength`)))))))))

(fn `Process Hits in Once Trace`
  (params (HitOuts :type "Array of HitResult Structure") (IsLeftIn :type Boolean) (IsRightIn :type Boolean))
  (locals (HasHitBlocker :type Boolean) (HitBlocker :type "/Game/BlueprintClasses/QuantumComponents/QuantumLight/BP_QuantumLightComponenent Object Reference") (Special :type Boolean :default false))
  (bind (_firsthitidlight _hitpanelsleft _hitpanelsright) (break `/Game/DataTypes/Structs/DataForPanelsInTrace` (`self.DataForPanels`)))
  (bind (_firsthitidlight_2 _hitpanelsleft_2 _hitpanelsright_2) (break `/Game/DataTypes/Structs/DataForPanelsInTrace` (`self.DataForPanels`)))
  (set `local.HasHitBlocker` false)
  (for _array_element HitOuts
    (bind (_bblockinghit _binitialoverlap _time _distance _location _impactpoint _normal _impactnormal _physmat _hitactor) (`GameplayStatics.BreakHitResult` _array_element))
    (bind _output_get (set `local.Special` (and (or (`local.IsLeftIn`) (`local.IsRightIn`)) _bblockinghit)))
    (if _output_get
      (`|ExecutionSequence` :!label _label
        (:`then_0`
          (if (or (`local.IsLeftIn`) (`local.IsRightIn`))
            (if (`local.Special`)
              (if (`local.IsLeftIn`) :!label _label_2
                (bind _returnvalue (+ _distance 10.0))
                (`KismetArrayLibrary.Array_Add` _hitpanelsleft_2 _returnvalue)
                (elif (`local.IsRightIn`)
                  (`KismetArrayLibrary.Array_Add` _hitpanelsright_2 _returnvalue)))
              (else
                (if (== _firsthitidlight -1)
                  (bind _idlightsource (`/Game/BlueprintClasses/QuantumComponents/QuantumLight/BP_QuantumLightComponenent.IdLightSource` (stale _asbp_quantum_light_componenent)))
                  (set `self.DataForPanels` (make `/Game/DataTypes/Structs/DataForPanelsInTrace` _idlightsource _hitpanelsleft _hitpanelsright)))
                (if (== _idlightsource _firsthitidlight)
                  (goto _label_2))))))
        (:`then_1`
          (set `local.HasHitBlocker` true)))
      (else
        (bind _asbp_quantum_light_componenent (cast `/Game/BlueprintClasses/QuantumComponents/QuantumLight/BP_QuantumLightComponenent` _hitactor)
          (:`then`
            (goto _label))
          (:`CastFailed`
            ;[1 1 1] HitQuantumDetector
            (bind _asquantum_light_detector (cast `/Game/BlueprintClasses/QuantumComponents/QuantumLightDetector` _hitactor))
            (if (not (`local.HasHitBlocker`))
              (`/Game/BlueprintClasses/QuantumComponents/QuantumLightDetector.HitWithQuantumLight` _asquantum_light_detector))))))))

(fn `ScaleLight`
  (bind _spotlight (`self.SpotLight`))
  (bind _returnvalue (/ (`KismetMathLibrary.Conv_IntToDouble` (`self.AngleRange`)) 2.0))
  (`LocalLightComponent.SetAttenuationRadius` (`self.SpotLight`) (`self.LineLength`))
  (`|ExecutionSequence`
    (:`then_0`
      (`SpotLightComponent.SetInnerConeAngle` _spotlight _returnvalue))
    (:`then_1`
      (`SpotLightComponent.SetOuterConeAngle` _spotlight _returnvalue))))

(fn `ScalePanelsToUnits`
  (params (LineLengthLeft :type "Float (double-precision)") (NewParamRight :type "Float (double-precision)"))
  (bind _returnvalue (/ NewParamRight 100.0))
  (bind _returnvalue_2 (/ LineLengthLeft 100.0))
  (bind _returnvalue_3 (/ LineLengthLeft 2.0))
  (bind _returnvalue_4 (/ NewParamRight 2.0))
  (bind _l_outside_panel (`self.L Outside Panel`))
  (bind _r_outside_panel (`self.R Outside Panel`))
  (bind _l_inside_panel (`self.L Inside Panel`))
  (bind _r_inside_panel (`self.R Inside Panel`))
  (bind (_relativescale3d_x _relativescale3d_y _relativescale3d_z) (`KismetMathLibrary.BreakVector` (`SceneComponent.RelativeScale3D` _l_outside_panel)))
  (bind (_relativescale3d_x_2 _relativescale3d_y_2 _relativescale3d_z_2) (`KismetMathLibrary.BreakVector` (`SceneComponent.RelativeScale3D` _r_outside_panel)))
  (bind (_relativescale3d_x_3 _relativescale3d_y_3 _relativescale3d_z_3) (`KismetMathLibrary.BreakVector` (`SceneComponent.RelativeScale3D` _r_inside_panel)))
  (bind (_relativescale3d_x_4 _relativescale3d_y_4 _relativescale3d_z_4) (`KismetMathLibrary.BreakVector` (`SceneComponent.RelativeScale3D` _l_inside_panel)))
  ;[1 1 1] Set Scale of Planes
  (`|ExecutionSequence`
    (:`then_0`
      (`SceneComponent.SetRelativeScale3D` _l_outside_panel (`KismetMathLibrary.MakeVector` _returnvalue_2 _relativescale3d_y _relativescale3d_z))
      (`SceneComponent.SetRelativeScale3D` _l_inside_panel (`KismetMathLibrary.MakeVector` _returnvalue_2 _relativescale3d_y_4 _relativescale3d_z_4))
      ;[1 1 1] Set Location of Planes
      (`SceneComponent.K2_SetRelativeLocation` (`self.L Outside Panel`) (`KismetMathLibrary.MakeVector` _returnvalue_3) false false)
      (`SceneComponent.K2_SetRelativeLocation` (`self.L Inside Panel`) (`KismetMathLibrary.MakeVector` _returnvalue_3) false false))
    (:`then_1`
      (`SceneComponent.SetRelativeScale3D` _r_outside_panel (`KismetMathLibrary.MakeVector` _returnvalue _relativescale3d_y_2 _relativescale3d_z_2))
      (`SceneComponent.SetRelativeScale3D` _r_inside_panel (`KismetMathLibrary.MakeVector` _returnvalue _relativescale3d_y_3 _relativescale3d_z_3))
      (`SceneComponent.K2_SetRelativeLocation` (`self.R Outside Panel`) (`KismetMathLibrary.MakeVector` _returnvalue_4) false false)
      (`SceneComponent.K2_SetRelativeLocation` (`self.R Inside Panel`) (`KismetMathLibrary.MakeVector` _returnvalue_4) false false))))

(fn `UserConstructionScript`
  (bind _linelength (`self.LineLength`))
  (bind _returnvalue (`KismetMathLibrary.Conv_IntToDouble` (`self.AngleRange`)))
  (`|ExecutionSequence`
    (:`then_0`
      ;[1 1 1] Set Yaw of planes / scenes
      (`|ExecutionSequence`
        (:`then_0`
          (`SceneComponent.K2_SetRelativeRotation` (`self.LeftSceneRoot`) (`KismetMathLibrary.MakeRotator` 0.0 0.0 (* _returnvalue -0.5)) false false))
        (:`then_1`
          (`SceneComponent.K2_SetRelativeRotation` (`self.RightSceneRoot`) (`KismetMathLibrary.MakeRotator` 0.0 0.0 (* _returnvalue 0.5)) false false))))
    (:`then_1`
      (`self.ScalePanelsToUnits` _linelength _linelength))
    (:`then_2`
      (`self.ScaleLight`))))