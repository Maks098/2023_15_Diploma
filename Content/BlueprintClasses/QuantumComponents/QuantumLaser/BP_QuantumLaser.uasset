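; A switchable coloured quantum laser that triggers QuantumLightDetectors of a matching colour, with white matching any colour.
; A looping timer, paused while off, runs multi line traces along the forward vector.
; Blocking hits, or overlapped lasers of a compatible colour, cut the beam short by rescaling its mesh, light and sparkles.
; The construction script sets initial length and applies the colour's material and light colour.
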(event `/Game/BlueprintClasses/OnOffInterface.TurnOn`
  (set `self.State` true)
  (`KismetSystemLibrary.K2_UnPauseTimerHandle` (`self.TimerHandle`))
  (`PrimitiveComponent.SetCollisionEnabled` (`self.LaserMesh`) "QueryOnly")
  (`SceneComponent.SetVisibility` (`self.LaserMesh`) (`self.State`) false :!label _label)
  (`SceneComponent.SetVisibility` (`self.Sparkles Placeholder`) (`self.State`) false)
  (`SceneComponent.SetVisibility` (`self.LaserLightSource`) (`self.State`) false))

(event `/Game/BlueprintClasses/OnOffInterface.TurnOff`
  (set `self.State` false)
  (`KismetSystemLibrary.K2_PauseTimerHandle` (`self.TimerHandle`))
  (`PrimitiveComponent.SetCollisionEnabled` (`self.LaserMesh`) "NoCollision")
  (goto _label))

(event `self.ReceiveBeginPlay`
  (bind _returnvalue (`KismetSystemLibrary.K2_SetTimer` null "ShootTraces" (/ 1.0 (`self.UpdateFrequency`)) true))
  (set `self.TimerHandle` _returnvalue)
  (if (not (`self.State`))
    (`self.TurnOff`)))

(fn `IsSameOrWhiteColour`
  (params (`Targets Colour` :type "/Game/BlueprintClasses/QuantumComponents/QuantumLaser/E_QuantumLaserTypes Enum" :default "NewEnumerator1"))
  (returns (MatchingColour :type Boolean))
  (bind _colour (`self.Colour`))
  (return (or (`|EnumEquality` "NewEnumerator3" `Targets Colour`) (`|EnumEquality` `Targets Colour` _colour) (`|EnumEquality` _colour "NewEnumerator3"))))

(fn `ProcessHitsInTrace`
  (params (TraceHits :type "Array of HitResult Structure"))
  (locals (HitBlocker :type Boolean))
  (for _array_element TraceHits
    (bind (_bblockinghit _binitialoverlap _time _distance _location _impactpoint _normal _impactnormal _physmat _hitactor) (`GameplayStatics.BreakHitResult` _array_element))
    (if _bblockinghit
      (bind _returnvalue (+ _distance 5.1))
      (`self.ScaleLaserMeshAndLight` _returnvalue)
      (bind _asquantum_light_detector (cast `/Game/BlueprintClasses/QuantumComponents/QuantumLightDetector/QuantumLightDetector` _hitactor)
        (:`then`
          (bind _matchingcolour (`self.IsSameOrWhiteColour` (`/Game/BlueprintClasses/QuantumComponents/QuantumLightDetector/QuantumLightDetector.Colour` _asquantum_light_detector)))
          (if _matchingcolour
            (`/Game/BlueprintClasses/QuantumComponents/QuantumLightDetector/QuantumLightDetector.HitWithQuantumLight` _asquantum_light_detector)))
        (:`CastFailed`
          _))
      (return)
      (else
        (bind _asbp_quantum_laser (cast `/Game/BlueprintClasses/QuantumComponents/QuantumLaser/BP_QuantumLaser` _hitactor))
        (bind _matchingcolour_2 (`self.IsSameOrWhiteColour` (`/Game/BlueprintClasses/QuantumComponents/QuantumLaser/BP_QuantumLaser.Colour` _asbp_quantum_laser)))
        (if _matchingcolour_2
          (`self.ScaleLaserMeshAndLight` _returnvalue)
          (return)))))
  (`self.ScaleLaserMeshAndLight` (`self.Laser Length`))
  (return))

(fn `ScaleLaserMeshAndLight`
  (params (Length :type "Float (double-precision)"))
  (bind _lasermesh (`self.LaserMesh`))
  (bind _laserlightsource (`self.LaserLightSource`))
  (bind _sparkles_placeholder (`self.Sparkles Placeholder`))
  (bind (_relativescale3d_x _relativescale3d_y) (`KismetMathLibrary.BreakVector` (`SceneComponent.RelativeScale3D` _lasermesh)))
  (bind (_relativelocation_x _relativelocation_y _relativelocation_z) (`KismetMathLibrary.BreakVector` (`SceneComponent.RelativeLocation` _lasermesh)))
  (bind (_relativelocation_x_2 _relativelocation_y_2 _relativelocation_z_2) (`KismetMathLibrary.BreakVector` (`SceneComponent.RelativeLocation` _sparkles_placeholder)))
  (bind (_relativelocation_x_3 _relativelocation_y_3 _relativelocation_z_3) (`KismetMathLibrary.BreakVector` (`SceneComponent.RelativeLocation` _laserlightsource)))
  (`|ExecutionSequence`
    (:`then_0`
      (`SceneComponent.SetRelativeScale3D` _lasermesh (`KismetMathLibrary.MakeVector` _relativescale3d_x _relativescale3d_y (/ Length 100.0)))
      (`SceneComponent.K2_SetRelativeLocation` _lasermesh (`KismetMathLibrary.MakeVector` (/ Length 2.0) _relativelocation_y _relativelocation_z) false false)
      (`SceneComponent.K2_SetRelativeLocation` _sparkles_placeholder (`KismetMathLibrary.MakeVector` Length _relativelocation_y_2 _relativelocation_z_2) false false))
    (:`then_1`
      (`PointLightComponent.SetSourceLength` _laserlightsource Length)
      (`SceneComponent.K2_SetRelativeLocation` _laserlightsource (`KismetMathLibrary.MakeVector` (/ Length 2.0) _relativelocation_y_3 _relativelocation_z_3) false false))))

(fn `ShootTraces`
  (bind _returnvalue (`self.K2_GetActorLocation`))
  (if (`self.State`)
    (bind _outhits (`KismetSystemLibrary.LineTraceMulti` :`Start` _returnvalue :`End` (+ _returnvalue (* (`self.GetActorForwardVector`) (`self.Laser Length`))) :`TraceChannel` "TraceTypeQuery3" :`DrawDebugType` (`self.Draw Debug Type`) :`DrawTime` (/ 1.0 (`self.UpdateFrequency`))))
    (`self.ProcessHitsInTrace` _outhits)))

(fn `UserConstructionScript`
  (bind _laserlightsource (`self.LaserLightSource`))
  (bind _lasermesh (`self.LaserMesh`))
  (`|ExecutionSequence`
    (:`then_0`
      (`self.ScaleLaserMeshAndLight` (`self.Laser Length`)))
    (:`then_1`
      (switch `/Game/BlueprintClasses/QuantumComponents/QuantumLaser/E_QuantumLaserTypes` (`self.Colour`)
        (:`NewEnumerator1`
          (`PrimitiveComponent.SetMaterial` _lasermesh 0 "/Game/BlueprintClasses/QuantumComponents/QuantumLaser/Materials/RedQuantumLaserMaterial.RedQuantumLaserMaterial")
          (`LightComponent.SetLightColor` _laserlightsource (make `LinearColor` 1.0 0.0 0.0 1.0) true))
        (:`NewEnumerator2`
          (`PrimitiveComponent.SetMaterial` _lasermesh 0 "/Game/BlueprintClasses/QuantumComponents/QuantumLaser/Materials/GreenQuantumLaserMaterial.GreenQuantumLaserMaterial")
          (`LightComponent.SetLightColor` _laserlightsource (make `LinearColor` 0.0 1.0 0.0 1.0) true))
        (:`NewEnumerator0`
          (`PrimitiveComponent.SetMaterial` _lasermesh 0 "/Game/BlueprintClasses/QuantumComponents/QuantumLaser/Materials/BlueQuantumLaserMaterial.BlueQuantumLaserMaterial")
          (`LightComponent.SetLightColor` _laserlightsource (make `LinearColor` 0.0 0.0 1.0 1.0) true))
        (:`NewEnumerator3`
          (`PrimitiveComponent.SetMaterial` _lasermesh 0 "/Game/BlueprintClasses/QuantumComponents/QuantumLaser/Materials/QuantumLaserMaterial.QuantumLaserMaterial")
          (`LightComponent.SetLightColor` _laserlightsource (make `LinearColor` 1.0 1.0 1.0 1.0) true))))))