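; Camera actor for a cutscene that, going by its name, follows the main menu.
; On BeginPlay it plays the FadeInWhite level sequence and makes itself the player's view target.
; Two timelines then run together, one driving the camera's relative X location and the other its pitch.
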(event `self.ReceiveBeginPlay`
  (bind (_outactor _returnvalue) (`LevelSequencePlayer.CreateLevelSequencePlayer` "/Game/BlueprintClasses/Dialogue/FadeInWhite.FadeInWhite"))
  (`MovieSceneSequencePlayer.Play` _returnvalue)
  (set `self.bFindCameraComponentWhenViewTarget` true)
  (`PlayerController.SetViewTargetWithBlend` (`GameplayStatics.GetPlayerController` 0) self 0.0 "VTBlend_Cubic" 0.0 false)
  (`|ExecutionSequence`
    (:`then_0`
      (bind (_direction _xposition) (`Timeline|Timeline_0`)
        (:`Update`
          (`SceneComponent.K2_SetRelativeLocation` (`self.Camera`) (`KismetMathLibrary.MakeVector` _xposition) false false))))
    (:`then_1`
      (bind (_direction_2 _yrotation) (`Timeline|RotationTimeline`)
        (:`Update`
          (`SceneComponent.K2_SetRelativeRotation` (`self.Camera`) (`KismetMathLibrary.MakeRotator` 0.0 _yrotation) false false))))))

(fn `UserConstructionScript`)