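; BP_Checkpoint is a checkpoint actor that registers itself as the player's last checkpoint when touched.
; A capsule overlap by BP_ThirdPersonCharacter sets the checkpoint on the character and requests a save message from the game instance.
; Each activation starts a cooldown, counted down on Tick, that blocks repeat triggers.
; ChangeAppearance swaps the base's core material between on and off by State, but is not called here.
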(event `self.ReceiveTick`
  (params (DeltaSeconds :type "Float (single-precision)"))
  (bind _currentcooldown (`self.CurrentCooldown`))
  (if (> _currentcooldown 0.0)
    (set `self.CurrentCooldown` (- _currentcooldown DeltaSeconds))))

(event `self.CapsuleCollision.OnComponentBeginOverlap`
  (params (OverlappedComponent :type "PrimitiveComponent Object Reference") (OtherActor :type "Actor Object Reference") (OtherComp :type "PrimitiveComponent Object Reference") (OtherBodyIndex :type Integer) (bFromSweep :type Boolean) (SweepResult :type "HitResult Structure (by ref)"))
  (if (not (> (`self.CurrentCooldown`) 0.0))
    (bind _asbp_third_person_character (cast `/Game/ThirdPerson/Blueprints/BP_ThirdPersonCharacter` OtherActor))
    (`/Game/ThirdPerson/Blueprints/BP_ThirdPersonCharacter.SetLastCheckpoint` _asbp_third_person_character self)
    (message `/Game/Save/BPI_Persistance.RequestSave` (`GameplayStatics.GetGameInstance`) true)
    (set `self.CurrentCooldown` (`self.CheckpointCooldown`))))

(fn `ChangeAppearance`
  (bind _base (`self.Base`))
  (if (`self.State`)
    (`PrimitiveComponent.SetMaterial` _base 2 "/Game/BlenderFiles/Materials/Detector/OnCoreWhite.OnCoreWhite")
    (else
      (`PrimitiveComponent.SetMaterial` _base 2 "/Game/BlenderFiles/Materials/Detector/OffCoreWhite.OffCoreWhite"))))

(fn `UserConstructionScript`)