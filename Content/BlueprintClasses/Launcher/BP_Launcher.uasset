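; BP_Launcher is a launch pad that throws the third-person character or an old box toward a Target actor.
; On box overlap it computes a custom-arc projectile velocity to the target, then launches the character with per-axis multipliers.
; Boxes are released, zeroed in velocity and given that velocity as an impulse.
; A red Niagara effect is aimed at the target in construction and on BeginPlay.
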(event `self.ReceiveBeginPlay`
  (`self.SetNiagaraRotation`))

(event `self.Box.OnComponentBeginOverlap`
  (params (OverlappedComponent :type "PrimitiveComponent Object Reference") (OtherActor :type "Actor Object Reference") (OtherComp :type "PrimitiveComponent Object Reference") (OtherBodyIndex :type Integer) (bFromSweep :type Boolean) (SweepResult :type "HitResult Structure (by ref)"))
  (bind _returnvalue (`self.K2_GetActorLocation` (`self.Target`)))
  (bind _asbp_third_person_character (cast `/Game/ThirdPerson/Blueprints/BP_ThirdPersonCharacter` OtherActor)
    (:`then`
      (bind _outlaunchvelocity (`GameplayStatics.SuggestProjectileVelocity_CustomArc` (`self.K2_GetActorLocation` OtherActor) _returnvalue (`self.Override Gravity Z`) (`self.Arc Param`)))
      (`Character.LaunchCharacter` _asbp_third_person_character (* _outlaunchvelocity (`KismetMathLibrary.MakeVector` (`self.Multiply X Velocity`) (`self.Multiply Y Velocity`) (`self.Multiply Z Velocity`))) true true))
    (:`CastFailed`
      (bind _asbp_old_box (cast `/Game/BlueprintClasses/BP_OldBox` OtherActor))
      (cast `StaticMeshComponent` OtherComp)
      (bind _outlaunchvelocity_2 (`GameplayStatics.SuggestProjectileVelocity_CustomArc` (`self.K2_GetActorLocation` _asbp_old_box) _returnvalue (`self.Override Gravity Z`) (`self.Arc Param`)))
      (`/Game/BlueprintClasses/BP_OldBox.Release Box` _asbp_old_box)
      (bind _staticmesh (`/Game/BlueprintClasses/BP_OldBox.StaticMesh` _asbp_old_box))
      (`PrimitiveComponent.SetPhysicsLinearVelocity` _staticmesh (0.0 0.0 0.0) false "None")
      (`PrimitiveComponent.AddImpulse` _staticmesh _outlaunchvelocity_2 "None" true))))

(fn `SetNiagaraRotation`
  (bind _ns_quantumlight_red (`self.NS_QuantumLight_Red`))
  (bind _target (`self.Target`))
  (bind (_returnvalue_roll _returnvalue_pitch _returnvalue_yaw) (`KismetMathLibrary.BreakRotator` (`KismetMathLibrary.FindLookAtRotation` (`self.K2_GetActorLocation`) (`self.K2_GetActorLocation` _target))))
  (if (`KismetSystemLibrary.IsValid` _target)
    (`SceneComponent.K2_SetRelativeRotation` _ns_quantumlight_red (`KismetMathLibrary.MakeRotator` (- 90.0 _returnvalue_pitch) 0.0 _returnvalue_yaw) false false)
    (else
      (`SceneComponent.K2_SetRelativeRotation` _ns_quantumlight_red (`KismetMathLibrary.MakeRotator` 0.0) false false))))

(fn `UserConstructionScript`
  (`self.SetNiagaraRotation`))