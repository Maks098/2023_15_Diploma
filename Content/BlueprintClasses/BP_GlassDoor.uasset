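; BP_GlassDoor is a two-panel glass door that slides open and closed through its Turnon and TurnOff events.
; Turnon plays two timelines in sequence, each setting one panel's relative X location, and TurnOff reverses both to retrace the motion.
; BeginPlay enables input from player controller 0, though the graph contains no input events.
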(event `self.ReceiveBeginPlay`
  (`self.EnableInput` (`GameplayStatics.GetPlayerController` 0)))

(event `/Game/BlueprintClasses/OnOffInterface.TurnOn`
  (`|ExecutionSequence`
    (:`then_0`
      (bind (_direction _0_2_sec) (`Timeline|Timeline` :!label _label)
        (:`Update`
          (`SceneComponent.K2_SetRelativeLocation` (`self.Left_door`) (`KismetMathLibrary.MakeVector` _0_2_sec) false false))))
    (:`then_1`
      (bind (_direction_2 _0_2_sec_2) (`Timeline|Door` :!label _label_2)
        (:`Update`
          (`SceneComponent.K2_SetRelativeLocation` (`self.Right_door`) (`KismetMathLibrary.MakeVector` _0_2_sec_2) false false))))))

(event `/Game/BlueprintClasses/OnOffInterface.TurnOff`
  (`|ExecutionSequence`
    (:`then_0`
      (goto _label :!via `Reverse`))
    (:`then_1`
      (goto _label_2 :!via `Reverse`))))

(fn `UserConstructionScript`)