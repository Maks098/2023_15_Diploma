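; BP_Doors is a double sliding door that opens and closes through its Turnon and TurnOff events.
; Turnon plays two timelines from the start, each setting the relative X of one panel, LeftDoor or RightDoor, without sweep.
; TurnOff reverses both timelines from the end, so an interrupted motion jumps rather than resuming.
; BeginPlay enables player 0 input, though the graph handles no input events.
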(event `self.ReceiveBeginPlay`
  (`self.EnableInput` (`GameplayStatics.GetPlayerController` 0)))

(event `/Game/BlueprintClasses/OnOffInterface.TurnOn`
  (`|ExecutionSequence`
    (:`then_0`
      (bind (_direction _0_2_sec) (`Timeline|Timeline` :!via `PlayFromStart` :!label _label)
        (:`Update`
          (`SceneComponent.K2_SetRelativeLocation` (`self.Left_door`) (`KismetMathLibrary.MakeVector` _0_2_sec) false false))))
    (:`then_1`
      (bind (_direction_2 _0_2_sec_2) (`Timeline|Door` :!via `PlayFromStart` :!label _label_2)
        (:`Update`
          (`SceneComponent.K2_SetRelativeLocation` (`self.Right_door`) (`KismetMathLibrary.MakeVector` _0_2_sec_2) false false))))))

(event `/Game/BlueprintClasses/OnOffInterface.TurnOff`
  (`|ExecutionSequence`
    (:`then_0`
      (goto _label :!via `ReverseFromEnd`))
    (:`then_1`
      (goto _label_2 :!via `ReverseFromEnd`))))

(fn `UserConstructionScript`)