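; Single sliding door that moves vertically and handles level streaming as it toggles.
; A timeline drives the door mesh's relative Z, starting on BeginPlay if IsOn is set, and plays an attenuated whoosh sound when finished.
; Turnon starts async loading of LevelToLoad and plays the timeline, while TurnOff unloads LevelToUnload and reverses it, neither waiting for streaming to complete.
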(event `self.ReceiveBeginPlay`
  (`self.EnableInput` (`GameplayStatics.GetPlayerController` 0))
  (if (`self.IsOn`)
    (bind (_direction _alpha) (`Timeline|Timeline` :!label _label)
      (:`Update`
        (`SceneComponent.K2_SetRelativeLocation` (`self.Door_Single_Door_Single`) (`KismetMathLibrary.MakeVector` 0.0 -100.0 _alpha) false false))
      (:`Finished`
        (`GameplayStatics.PlaySoundAtLocation` "/Game/Audio/light-whoosh-241728.light-whoosh-241728" (`self.K2_GetActorLocation`) (struct) 1.0 1.0 0.0 "/Game/Audio/SoundAttenuationSFX.SoundAttenuationSFX" null null null)))))

(event `self.TurnOn`
  (`GameplayStatics.LoadStreamLevel` (`KismetStringLibrary.Conv_StringToName` (`self.LevelToLoad`)) true)
  (goto _label))

(event `self.TurnOff`
  (`GameplayStatics.UnloadStreamLevel` (`KismetStringLibrary.Conv_StringToName` (`self.LevelToUnload`)))
  (goto _label :!via `Reverse`))

(fn `UserConstructionScript`)