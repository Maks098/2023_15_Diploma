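; Double sliding door actor that opens on Turnon and closes on TurnOff.
; Two timelines, DoorR and DoorL, play or reverse together, each setting its door panel's relative X location from its Alpha track.
; Both timelines share one Finished path that plays an attenuated whoosh sound at the actor's location.
; BeginPlay enables input from player controller 0, though the graph has no input events.
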(event `self.ReceiveBeginPlay`
  (`self.EnableInput` (`GameplayStatics.GetPlayerController` 0)))

(event `/Game/BlueprintClasses/OnOffInterface.TurnOn`
  (`|ExecutionSequence`
    (:`then_0`
      (bind (_direction _alpha) (`Timeline|DoorR` :!label _label)
        (:`Update`
          (`SceneComponent.K2_SetRelativeLocation` (`self.Door_Double_Door_Double_R`) (`KismetMathLibrary.MakeVector` _alpha) false false))
        (:`Finished`
          (`GameplayStatics.PlaySoundAtLocation` "/Game/Audio/light-whoosh-241728.light-whoosh-241728" (`self.K2_GetActorLocation`) (struct) 1.0 1.0 0.0 "/Game/Audio/SoundAttenuationSFX.SoundAttenuationSFX" null null null :!label _label_2))))
    (:`then_1`
      (bind (_direction_2 _alpha_2) (`Timeline|DoorL` :!label _label_3)
        (:`Update`
          (`SceneComponent.K2_SetRelativeLocation` (`self.Door_Double_Door_Double_L`) (`KismetMathLibrary.MakeVector` _alpha_2) false false))
        (:`Finished`
          (goto _label_2))))))

(event `/Game/BlueprintClasses/OnOffInterface.TurnOff`
  (`|ExecutionSequence`
    (:`then_0`
      (goto _label :!via `Reverse`))
    (:`then_1`
      (goto _label_3 :!via `Reverse`))))

(fn `UserConstructionScript`)