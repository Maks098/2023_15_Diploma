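; BP_AppearingSignsOnComputer is an actor holding a group of static mesh signs, named as appearing on a computer, that stay invisible until triggered.
; BeginPlay hides all the mesh components in game.
; The Turnon event unhides the same set all at once, with no animation or delay, and nothing in this Blueprint calls it or hides them again.
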(event `self.ReceiveBeginPlay`
  (`SceneComponent.SetHiddenInGame` (`self.StaticMesh17`) true false)
  (`SceneComponent.SetHiddenInGame` (`self.StaticMesh13`) true false)
  (`SceneComponent.SetHiddenInGame` (`self.StaticMesh8`) true false)
  (`SceneComponent.SetHiddenInGame` (`self.StaticMesh11`) true false)
  (`SceneComponent.SetHiddenInGame` (`self.StaticMesh12`) true false)
  (`SceneComponent.SetHiddenInGame` (`self.StaticMesh14`) true false)
  (`SceneComponent.SetHiddenInGame` (`self.StaticMesh15`) true false)
  (`SceneComponent.SetHiddenInGame` (`self.StaticMesh16`) true false)
  (`SceneComponent.SetHiddenInGame` (`self.StaticMesh18`) true false)
  (`SceneComponent.SetHiddenInGame` (`self.StaticMesh10`) true false)
  (`SceneComponent.SetHiddenInGame` (`self.StaticMesh9`) true false)
  (`SceneComponent.SetHiddenInGame` (`self.StaticMesh2`) true false)
  (`SceneComponent.SetHiddenInGame` (`self.StaticMesh1`) true false)
  (`SceneComponent.SetHiddenInGame` (`self.StaticMesh`) true false)
  (`SceneComponent.SetHiddenInGame` (`self.StaticMesh3`) true false)
  (`SceneComponent.SetHiddenInGame` (`self.StaticMesh7`) true false)
  (`SceneComponent.SetHiddenInGame` (`self.StaticMesh4`) true false)
  (`SceneComponent.SetHiddenInGame` (`self.StaticMesh5`) true false)
  (`SceneComponent.SetHiddenInGame` (`self.StaticMesh6`) true false))

(event `/Game/BlueprintClasses/OnOffInterface.TurnOn`
  (`SceneComponent.SetHiddenInGame` (`self.StaticMesh8`) false false)
  (`SceneComponent.SetHiddenInGame` (`self.StaticMesh11`) false false)
  (`SceneComponent.SetHiddenInGame` (`self.StaticMesh12`) false false)
  (`SceneComponent.SetHiddenInGame` (`self.StaticMesh13`) false false)
  (`SceneComponent.SetHiddenInGame` (`self.StaticMesh14`) false false)
  (`SceneComponent.SetHiddenInGame` (`self.StaticMesh15`) false false)
  (`SceneComponent.SetHiddenInGame` (`self.StaticMesh16`) false false)
  (`SceneComponent.SetHiddenInGame` (`self.StaticMesh17`) false false)
  (`SceneComponent.SetHiddenInGame` (`self.StaticMesh18`) false false)
  (`SceneComponent.SetHiddenInGame` (`self.StaticMesh10`) false false)
  (`SceneComponent.SetHiddenInGame` (`self.StaticMesh9`) false false)
  (`SceneComponent.SetHiddenInGame` (`self.StaticMesh2`) false false)
  (`SceneComponent.SetHiddenInGame` (`self.StaticMesh1`) false false)
  (`SceneComponent.SetHiddenInGame` (`self.StaticMesh`) false false)
  (`SceneComponent.SetHiddenInGame` (`self.StaticMesh3`) false false)
  (`SceneComponent.SetHiddenInGame` (`self.StaticMesh7`) false false)
  (`SceneComponent.SetHiddenInGame` (`self.StaticMesh4`) false false)
  (`SceneComponent.SetHiddenInGame` (`self.StaticMesh5`) false false)
  (`SceneComponent.SetHiddenInGame` (`self.StaticMesh6`) false false))

(fn `UserConstructionScript`)