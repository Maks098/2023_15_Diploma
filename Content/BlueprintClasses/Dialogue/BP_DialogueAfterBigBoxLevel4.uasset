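; Dialogue actor, named for the moment after Level 4's big box, that shows NPC lines in a DialogueUI widget.
; A box overlap caches the third-person character, and Turnon stops its movement, enables input and creates the widget.
; E or left click advances the text row through a resettable DoOnce.
; After the last row it removes the widget, calls TurnOn on a linked Interactable and disables its input.
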(event `Key|E`
  (params (Key :type "Key Structure"))
  (:`Pressed`
    (`self.EventDialogueOccurs` :!label _label)))

(event `Key|LeftMouseButton`
  (params (Key :type "Key Structure"))
  (:`Pressed`
    (goto _label)))

(event `self.TurnOn`
  (`self.EnableInput` (`GameplayStatics.GetPlayerController` 0))
  (`/Game/ThirdPerson/Blueprints/BP_ThirdPersonCharacter.TurnOffMovement` (`self.Player`))
  (`self.EventDialogueOccurs`)
  (bind _returnvalue (`|CreateWidget` "/Game/BlueprintClasses/Dialogue/DialogueUI.DialogueUI_C"))
  (bind _output_get (set `self.Dialogue UI` _returnvalue))
  (`UserWidget.AddToViewport` _output_get 0)
  (for _ (`self.NPCText`)
    (`self.EventDialogueOccurs`)
    (break)))

(event `self.Box.OnComponentBeginOverlap`
  (params (OverlappedComponent :type "PrimitiveComponent Object Reference") (OtherActor :type "Actor Object Reference") (OtherComp :type "PrimitiveComponent Object Reference") (OtherBodyIndex :type Integer) (bFromSweep :type Boolean) (SweepResult :type "HitResult Structure (by ref)"))
  (bind _asbp_third_person_character (cast `/Game/ThirdPerson/Blueprints/BP_ThirdPersonCharacter` OtherActor))
  (set `self.Player` _asbp_third_person_character))

(event `self.EventDialogueOccurs`
  (bind _npctext (`self.NPCText`))
  (bind _textrow (`/Game/BlueprintClasses/Dialogue/DialogueUI.TextRow` (`self.Dialogue UI`)))
  (bind _returnvalue (+ _textrow 1))
  (`/Engine/EditorBlueprintResources/StandardMacros.DoOnce` false :!label _label_2
    (:`Completed`
      (set `/Game/BlueprintClasses/Dialogue/DialogueUI.Text` (`self.NPCText`) (`self.Dialogue UI`))
      (`Widget.SetVisibility` (`/Game/BlueprintClasses/Dialogue/DialogueUI.Image_0` (`self.Dialogue UI`)) "Visible")
      (`Widget.SetVisibility` (`/Game/BlueprintClasses/Dialogue/DialogueUI.TextBlock_0` (`self.Dialogue UI`)) "Visible")
      (if (> _returnvalue (- (`KismetArrayLibrary.Array_Length` _npctext) 1))
        (`Widget.RemoveFromParent` (`self.Dialogue UI`))
        (`self.ResetDialogue`)
        (if (== _textrow (- (`KismetArrayLibrary.Array_Length` _npctext) 1))
          (`Widget.SetVisibility` (`/Game/BlueprintClasses/Dialogue/DialogueUI.Image_0` (`self.Dialogue UI`)) "Hidden")
          (`Widget.SetVisibility` (`/Game/BlueprintClasses/Dialogue/DialogueUI.TextBlock_0` (`self.Dialogue UI`)) "Hidden")
          (`/Game/BlueprintClasses/OnOffInterface.TurnOn` (`self.Interactable`))
          (`self.DisableInput` (`GameplayStatics.GetPlayerController` 0)))
        (else
          (set `/Game/BlueprintClasses/Dialogue/DialogueUI.TextRow` _returnvalue (`self.Dialogue UI`))
          (`self.ResetDialogue`))))))

(event `ResetDialogue`
  (goto _label_2 :!via `Reset`))

(fn `UserConstructionScript`)