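; Work-in-progress dialogue actor, named for use after the big box level, that shows NPC text while cutting through cameras.
; Turnon enables input, turns off player movement and creates the DialogueUI widget.
; Space, E or left click advances the text row through a self-resetting DoOnce and moves the view to the next camera in CamerasToChange.
; After the last row it removes the widget, turns on Interactable and disables its input.
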(event `Key|SpaceBar`
  (params (Key :type "Key Structure"))
  (:`Pressed`
    (`self.EventDialogueOccurs` :!label _label)
    (`self.Event Change Camera`)
    (`KismetSystemLibrary.PrintString` "Hello")))

(event `Key|E`
  (params (Key :type "Key Structure"))
  (:`Pressed`
    (goto _label)))

(event `Key|LeftMouseButton`
  (params (Key :type "Key Structure"))
  (:`Pressed`
    (goto _label)))

(event `self.TurnOn`
  (`self.EnableInput` (`GameplayStatics.GetPlayerController` 0))
  (`/Game/ThirdPerson/Blueprints/BP_ThirdPersonCharacter.TurnOffMovement` (`self.Player`))
  (`self.EventDialogueOccurs`)
  (bind _returnvalue (`|CreateWidget` "/Game/BlueprintClasses/Dialogue/DialogueUI.DialogueUI_C"))
  (bind _output_get (set `self.Dialogue UI` _returnvalue))
  (`UserWidget.AddToViewport` _output_get 0)
  (for _ (`self.NPCText`)
    (`self.EventDialogueOccurs`)
    (break)))

(event `self.ReceiveBeginPlay`
  (bind _returnvalue (`GameplayStatics.GetActorOfClass` "/Game/ThirdPerson/Blueprints/BP_ThirdPersonCharacter.BP_ThirdPersonCharacter_C"))
  (set `self.Player` _returnvalue)
  (set `self.CameraIndex` 0))

(event `Event Change Camera`
  (`PlayerController.SetViewTargetWithBlend` (`GameplayStatics.GetPlayerController` 0) (`|GetArrayItem` (`self.CamerasToChange`) (`self.CameraIndex`)) 0.0 "VTBlend_Linear" 0.0 false)
  (set `self.CameraIndex` (+ (`self.CameraIndex`) 1)))

(event `self.EventDialogueOccurs`
  (bind _npctext (`self.NPCText`))
  (bind _textrow (`/Game/BlueprintClasses/Dialogue/DialogueUI.TextRow` (`self.Dialogue UI`)))
  (bind _returnvalue (+ _textrow 1))
  (`/Engine/EditorBlueprintResources/StandardMacros.DoOnce` false :!label _label_2
    (:`Completed`
      (set `/Game/BlueprintClasses/Dialogue/DialogueUI.Text` (`self.NPCText`) (`self.Dialogue UI`))
      (`Widget.SetVisibility` (`/Game/BlueprintClasses/Dialogue/DialogueUI.Image_0` (`self.Dialogue UI`)) "Visible")
      (`Widget.SetVisibility` (`/Game/BlueprintClasses/Dialogue/DialogueUI.TextBlock_0` (`self.Dialogue UI`)) "Visible")
      (if (> _returnvalue (- (`KismetArrayLibrary.Array_Length` _npctext) 1))
        (`Widget.RemoveFromParent` (`self.Dialogue UI`))
        (`self.ResetDialogue`)
        (if (== _textrow (- (`KismetArrayLibrary.Array_Length` _npctext) 1))
          (`Widget.SetVisibility` (`/Game/BlueprintClasses/Dialogue/DialogueUI.Image_0` (`self.Dialogue UI`)) "Hidden")
          (`Widget.SetVisibility` (`/Game/BlueprintClasses/Dialogue/DialogueUI.TextBlock_0` (`self.Dialogue UI`)) "Hidden")
          (`/Game/BlueprintClasses/OnOffInterface.TurnOn` (`self.Interactable`))
          (`self.DisableInput` (`GameplayStatics.GetPlayerController` 0)))
        (else
          (set `/Game/BlueprintClasses/Dialogue/DialogueUI.TextRow` _returnvalue (`self.Dialogue UI`))
          (`self.ResetDialogue`))))))

(event `ResetDialogue`
  (goto _label_2 :!via `Reset`))

(fn `UserConstructionScript`)