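; Level 1 trigger actor that runs a one-time dialogue with Odumani, then moves the game to StageToOpen.
; Box overlap by the player enables input, creates DialogueUI, messages the first overlapping Dialogueable actor and starts the dialogue.
; Space, E or left click turns off movement and steps through NPCText, with a DoOnce reset after each step.
; After the last row it plays a fade-out sequence, briefly shows a widget and opens the level.
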(event `Key|SpaceBar`
  (params (Key :type "Key Structure"))
  (:`Pressed`
    (`/Game/ThirdPerson/Blueprints/BP_ThirdPersonCharacter.TurnOffMovement` (`self.Player`) :!label _label)
    (`self.EventDialogueOccurs`)))

(event `Key|E`
  (params (Key :type "Key Structure"))
  (:`Pressed`
    (goto _label)))

(event `self.ReceiveBeginPlay`
  (set `self.DidDialogueOccure?` false)
  (bind _returnvalue (`GameplayStatics.GetActorOfClass` "/Game/ThirdPerson/Blueprints/BP_ThirdPersonCharacter.BP_ThirdPersonCharacter_C"))
  (set `self.Player` _returnvalue))

(event `Key|LeftMouseButton`
  (params (Key :type "Key Structure"))
  (:`Pressed`
    (goto _label)))

(event `self.Box.OnComponentBeginOverlap`
  (params (OverlappedComponent :type "PrimitiveComponent Object Reference") (OtherActor :type "Actor Object Reference") (OtherComp :type "PrimitiveComponent Object Reference") (OtherBodyIndex :type Integer) (bFromSweep :type Boolean) (SweepResult :type "HitResult Structure (by ref)"))
  (if (not (`self.DidDialogueOccure?`))
    (set `self.DidDialogueOccure?` true)
    (cast `/Game/ThirdPerson/Blueprints/BP_ThirdPersonCharacter` OtherActor)
    (`|ExecutionSequence`
      (:`then_0`
        (`self.EnableInput` (`GameplayStatics.GetPlayerController` 0))
        (bind _returnvalue (`|CreateWidget` "/Game/BlueprintClasses/Dialogue/DialogueUI.DialogueUI_C"))
        (bind _output_get (set `self.DialogueUI` _returnvalue))
        (`UserWidget.AddToViewport` (`self.DialogueUI`) 10)
        (`UserWidget.AddToViewport` _output_get 10)
        (for _array_element (`self.GetOverlappingActors` null)
          (if (`KismetSystemLibrary.DoesImplementInterface` _array_element "/Game/BlueprintClasses/Dialogue/Dialogueable.Dialogueable_C")
            (message `/Game/BlueprintClasses/Dialogue/Dialogueable.EventDialogueOccurs` _array_element)
            (break))))
      (:`then_1`
        (goto _label)))))

(event `self.EventDialogueOccurs`
  (bind _npctext (`self.NPCText`))
  (bind _textrow (`/Game/BlueprintClasses/Dialogue/DialogueUI.TextRow` (`self.DialogueUI`)))
  (bind _returnvalue (+ _textrow 1))
  (`/Engine/EditorBlueprintResources/StandardMacros.DoOnce` false :!label _label_2
    (:`Completed`
      (set `/Game/BlueprintClasses/Dialogue/DialogueUI.Text` (`self.NPCText`) (`self.DialogueUI`))
      (`Widget.SetVisibility` (`/Game/BlueprintClasses/Dialogue/DialogueUI.Image_0` (`self.DialogueUI`)) "Visible")
      (`Widget.SetVisibility` (`/Game/BlueprintClasses/Dialogue/DialogueUI.TextBlock_0` (`self.DialogueUI`)) "Visible")
      (if (> _returnvalue (- (`KismetArrayLibrary.Array_Length` _npctext) 1))
        (`Widget.RemoveFromParent` (`self.DialogueUI`))
        (`self.ResetDialogue`)
        (if (== _textrow (- (`KismetArrayLibrary.Array_Length` _npctext) 1))
          (`Widget.SetVisibility` (`/Game/BlueprintClasses/Dialogue/Level1/RoomSearchPopup.Image_44` (`self.RoomSearchPopUp`)) "Hidden")
          (`Widget.SetVisibility` (`/Game/BlueprintClasses/Dialogue/Level1/RoomSearchPopup.TextBlock` (`self.RoomSearchPopUp`)) "Hidden")
          (`self.DisableInput` (`GameplayStatics.GetPlayerController` 0))
          (bind _outactor (`LevelSequencePlayer.CreateLevelSequencePlayer` "/Game/BlueprintClasses/Dialogue/FadeOutConst.FadeOutConst"))
          (`MovieSceneSequencePlayer.Play` (`LevelSequenceActor.SequencePlayer` _outactor))
          (bind _returnvalue_2 (`|CreateWidget` (`self.Widget`)))
          (`KismetSystemLibrary.Delay` 1.5)
          (`UserWidget.AddToViewport` _returnvalue_2 0)
          (`KismetSystemLibrary.Delay` 5.0)
          (`Widget.SetVisibility` _returnvalue_2 "Hidden")
          (`GameplayStatics.OpenLevel` (`self.StageToOpen`)))
        (else
          (set `/Game/BlueprintClasses/Dialogue/DialogueUI.TextRow` _returnvalue (`self.DialogueUI`))
          (`self.ResetDialogue`))))))

(event `ResetDialogue`
  (goto _label_2 :!via `Reset`))

(fn `UserConstructionScript`)