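; Level 1 final dialogue actor that plays NPC lines in a widget with timed staging.
; Turnon enables input, creates the UI, messages the first overlapping Dialogueable actor and stops player movement.
; Space, E or left click advances text through a resettable DoOnce, with click counts triggering a camera switch and light reveal.
; After the last row it removes the UI, disables input, restores the default camera and turns on NextDialogue.
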(event `Key|SpaceBar`
  (params (Key :type "Key Structure"))
  (:`Pressed`
    (set `self.ClicksCounter` (+ (`self.ClicksCounter`) 1) :!label _label)
    (`/Game/ThirdPerson/Blueprints/BP_ThirdPersonCharacter.TurnOffMovement` (`self.Player`) :!label _label_2)
    (`self.EventDialogueOccurs`)
    (`|ExecutionSequence`
      (:`then_0`
        (if (== (`self.ClicksCounter`) (`self.AfterHowManyClicksChangeCamera`))
          (`PlayerController.SetViewTargetWithBlend` (`GameplayStatics.GetPlayerController` 0) (`self.CameraToChange`) 0.0 "VTBlend_Linear" 0.0 false)))
      (:`then_1`
        (if (== (`self.ClicksCounter`) (`self.AfterHowManyClicksTurnOnLight`))
          (`SceneComponent.SetVisibility` (`Actor.RootComponent` (`self.LightToTurnOn`)) true false))))))

(event `Key|E`
  (params (Key :type "Key Structure"))
  (:`Pressed`
    (goto _label)))

(event `self.ReceiveBeginPlay`
  (`SceneComponent.SetVisibility` (`Actor.RootComponent` (`self.LightToTurnOn`)) false false)
  (set `self.ClicksCounter` 0)
  (bind _returnvalue (`GameplayStatics.GetActorOfClass` "/Game/ThirdPerson/Blueprints/BP_ThirdPersonCharacter.BP_ThirdPersonCharacter_C"))
  (set `self.Player` _returnvalue))

(event `Key|LeftMouseButton`
  (params (Key :type "Key Structure"))
  (:`Pressed`
    (goto _label)))

(event `/Game/BlueprintClasses/OnOffInterface.TurnOn`
  (`|ExecutionSequence`
    (:`then_0`
      (`self.EnableInput` (`GameplayStatics.GetPlayerController` 0))
      (bind _returnvalue (`|CreateWidget` "/Game/BlueprintClasses/Dialogue/DialogueUI.DialogueUI_C"))
      (bind _output_get (set `self.DialogueUI` _returnvalue))
      (`UserWidget.AddToViewport` (`self.DialogueUI`) 10)
      (`UserWidget.AddToViewport` _output_get 10)
      (for _array_element (`self.GetOverlappingActors` null)
        (if (`KismetSystemLibrary.DoesImplementInterface` _array_element "/Game/BlueprintClasses/Dialogue/Dialogueable.Dialogueable_C")
          (message `/Game/BlueprintClasses/Dialogue/Dialogueable.EventDialogueOccurs` _array_element)
          (break))))
    (:`then_1`
      (goto _label_2))))

(event `self.EventDialogueOccurs`
  (bind _returnvalue (`GameplayStatics.GetPlayerController` 0))
  (bind _npctext (`self.NPCText`))
  (bind _textrow (`/Game/BlueprintClasses/Dialogue/DialogueUI.TextRow` (`self.DialogueUI`)))
  (bind _returnvalue_2 (+ _textrow 1))
  (`/Engine/EditorBlueprintResources/StandardMacros.DoOnce` false :!label _label_3
    (:`Completed`
      (set `/Game/BlueprintClasses/Dialogue/DialogueUI.Text` (`self.NPCText`) (`self.DialogueUI`))
      (`Widget.SetVisibility` (`/Game/BlueprintClasses/Dialogue/DialogueUI.Image_0` (`self.DialogueUI`)) "Visible")
      (`Widget.SetVisibility` (`/Game/BlueprintClasses/Dialogue/DialogueUI.TextBlock_0` (`self.DialogueUI`)) "Visible")
      (if (> _returnvalue_2 (- (`KismetArrayLibrary.Array_Length` _npctext) 1))
        (`Widget.RemoveFromParent` (`self.DialogueUI`))
        (`self.ResetDialogue`)
        (if (== _textrow (- (`KismetArrayLibrary.Array_Length` _npctext) 1))
          (`self.DisableInput` _returnvalue)
          (`PlayerController.SetViewTargetWithBlend` _returnvalue (`self.DefaultCamera`) 0.0 "VTBlend_Linear" 0.0 false)
          (`self.TurnOn` (`self.NextDialogue`)))
        (else
          (set `/Game/BlueprintClasses/Dialogue/DialogueUI.TextRow` _returnvalue_2 (`self.DialogueUI`))
          (`self.ResetDialogue`))))))

(event `ResetDialogue`
  (goto _label_3 :!via `Reset`))

(fn `UserConstructionScript`)