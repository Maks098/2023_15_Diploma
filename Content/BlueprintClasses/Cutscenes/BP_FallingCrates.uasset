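; BP_FallingCrates is a scripted prop that animates a crate falling when the third-person character enters its trigger box.
; The box overlap plays a first timeline that drives the crate's relative location and yaw.
; When it finishes, a second timeline holds X and yaw fixed while animating Y, Z and roll, so the motion is keyframed in two stages without using physics.
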(event `self.Box.OnComponentBeginOverlap`
  (params (OverlappedComponent :type "PrimitiveComponent Object Reference") (OtherActor :type "Actor Object Reference") (OtherComp :type "PrimitiveComponent Object Reference") (OtherBodyIndex :type Integer) (bFromSweep :type Boolean) (SweepResult :type "HitResult Structure (by ref)"))
  (cast `/Game/ThirdPerson/Blueprints/BP_ThirdPersonCharacter` OtherActor)
  (bind (_direction _z _y _x _zrotation) (`Timeline|Timeline`)
    (:`Update`
      (`|ExecutionSequence`
        (:`then_0`
          (`SceneComponent.K2_SetRelativeLocation` (`self.Props_CrateLong_Props_CrateLong2`) (`KismetMathLibrary.MakeVector` _x _y _z) false false))
        (:`then_1`
          (`SceneComponent.K2_SetRelativeRotation` (`self.Props_CrateLong_Props_CrateLong2`) (`KismetMathLibrary.MakeRotator` 0.0 0.0 _zrotation) false false))))
    (:`Finished`
      (bind (_direction_2 _z_2 _y_2 _rotation) (`Timeline|Timeline_0`)
        (:`Update`
          (`|ExecutionSequence`
            (:`then_0`
              (`SceneComponent.K2_SetRelativeLocation` (`self.Props_CrateLong_Props_CrateLong2`) (`KismetMathLibrary.MakeVector` 190.0 _y_2 _z_2) false false))
            (:`then_1`
              (`SceneComponent.K2_SetRelativeRotation` (`self.Props_CrateLong_Props_CrateLong2`) (`KismetMathLibrary.MakeRotator` _rotation 0.0 -30.0) false false))))))))

(fn `UserConstructionScript`)