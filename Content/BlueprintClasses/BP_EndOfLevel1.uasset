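; BP_EndOfLevel1 is the level 1 exit trigger actor that shows a text prompt and lets the player end the level.
; Overlap by BP_ThirdPersonCharacter enables input on the actor and reveals the TextRender, which starts hidden; end overlap hides it but never disables input.
; Pressing E creates the FinishOfLevel1_Widget, shows the mouse cursor and pauses the game.
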(event `Key|E`
  (params (Key :type "Key Structure"))
  (:`Pressed`
    (bind _returnvalue (`|CreateWidget` "/Game/Widgets/FinishOfLevel1_Widget.FinishOfLevel1_Widget_C"))
    (`UserWidget.AddToViewport` _returnvalue 0)
    (set `PlayerController.bShowMouseCursor` true (`GameplayStatics.GetPlayerController` 0))
    (`GameplayStatics.SetGamePaused` true)))

(event `self.ReceiveBeginPlay`
  (`SceneComponent.SetVisibility` (`self.TextRender`) false false))

(event `self.ReceiveActorBeginOverlap`
  (params (OtherActor :type "Actor Object Reference"))
  (cast `/Game/ThirdPerson/Blueprints/BP_ThirdPersonCharacter` OtherActor)
  (`|ExecutionSequence`
    (:`then_0`
      (`self.EnableInput` (`GameplayStatics.GetPlayerController` 0)))
    (:`then_1`
      (bind _output_get (set `self.TextVisible` true))
      (if (`self.TextVisible`) :!label _label
        (`SceneComponent.SetVisibility` (`self.TextRender`) true false)
        (else
          (`SceneComponent.SetVisibility` (`self.TextRender`) false false))))))

(event `self.ReceiveActorEndOverlap`
  (params (OtherActor :type "Actor Object Reference"))
  (cast `/Game/ThirdPerson/Blueprints/BP_ThirdPersonCharacter` OtherActor)
  (bind _output_get (set `self.TextVisible` false))
  (goto _label))

(fn `UserConstructionScript`)