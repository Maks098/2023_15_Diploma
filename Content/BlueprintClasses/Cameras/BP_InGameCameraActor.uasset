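; In-game camera actor Blueprint that supplies a reference rotation for player controls through a MovementDirection component.
; The construction script aligns that component to the camera's world rotation when FollowCameraRotation is set, otherwise to a fixed yaw from ArrowRotation with zero pitch and roll.
; GetControlsRotation returns the component's world rotation, so the control direction can differ from the camera view.
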(fn `Get Controls Rotation`
  (returns (`Controls Rotation` :type "Rotator Structure"))
  (return (`SceneComponent.K2_GetComponentRotation` (`self.MovementDirection`))))

(fn `UserConstructionScript`
  (if (`self.FollowCameraRotation`)
    (`SceneComponent.K2_SetWorldRotation` (`self.MovementDirection`) (`SceneComponent.K2_GetComponentRotation` (`self.CameraComponent`)) false false)
    (else
      (`SceneComponent.K2_SetWorldRotation` (`self.MovementDirection`) (`KismetMathLibrary.MakeRotator` 0.0 0.0 (`self.ArrowRotation`)) false false))))