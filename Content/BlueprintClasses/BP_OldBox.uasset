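; A physics box that the third-person character can grab and drag around while standing inside its trigger box.
; Grabbing snaps the character to the nearest of four side points placed from the trigger extents, then activates a physics constraint to the box, slows walking and lightens the mass.
; Release or constraint breakage restores speed and heavy mass; breakage also zeroes velocity.
; Construction also attaches an optional quantum light detector.
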(event `On Box Released`
  (if (`self.canPlayerInteract?`)
    (`self.Release Box`)))

(event `On Box Grabbed`
  (if (`self.canPlayerInteract?`)
    (`self.Set Player Grabbing Position`)
    (`KismetSystemLibrary.DelayUntilNextTick`)
    (`self.Grab Box`)))

(event `self.Box.OnComponentBeginOverlap`
  (params (OverlappedComponent :type "PrimitiveComponent Object Reference") (OtherActor :type "Actor Object Reference") (OtherComp :type "PrimitiveComponent Object Reference") (OtherBodyIndex :type Integer) (bFromSweep :type Boolean) (SweepResult :type "HitResult Structure (by ref)"))
  (bind _asbp_third_person_character (cast `/Game/ThirdPerson/Blueprints/BP_ThirdPersonCharacter` OtherActor))
  (set `self.canPlayerInteract?` true)
  (set `self.Character Reference` _asbp_third_person_character))

(event `self.Box.OnComponentEndOverlap`
  (params (OverlappedComponent :type "PrimitiveComponent Object Reference") (OtherActor :type "Actor Object Reference") (OtherComp :type "PrimitiveComponent Object Reference") (OtherBodyIndex :type Integer))
  (cast `/Game/ThirdPerson/Blueprints/BP_ThirdPersonCharacter` OtherActor)
  (set `self.canPlayerInteract?` false))

(event `self.ReceiveBeginPlay`
  (`ActorComponent.Deactivate` (`self.PhysicsConstraint`)))

(event `self.PhysicsConstraint.OnConstraintBroken`
  (params (ConstraintIndex :type Integer))
  (bind _staticmesh (`self.StaticMesh`))
  (`self.Release Box`)
  (`PrimitiveComponent.SetAllPhysicsLinearVelocity` _staticmesh (0.0 0.0 0.0) false)
  (`PrimitiveComponent.SetAllPhysicsAngularVelocityInDegrees` _staticmesh (0.0 0.0 0.0) false))

(fn `Grab Box`
  (bind _charactermovement (`Character.CharacterMovement` (`self.Character Reference`)))
  (`PhysicsConstraintComponent.SetConstrainedComponents` (`self.PhysicsConstraint`) (`/Game/ThirdPerson/Blueprints/BP_ThirdPersonCharacter.StaticMesh` (`self.Character Reference`)) "None" (`self.StaticMesh`) "None")
  (`ActorComponent.Activate` (`self.PhysicsConstraint`) false)
  (set `CharacterMovementComponent.bOrientRotationToMovement` false _charactermovement)
  (set `self.Character Default Max Walk Speed` (`CharacterMovementComponent.MaxWalkSpeed` _charactermovement))
  (set `CharacterMovementComponent.MaxWalkSpeed` 140.0 _charactermovement)
  (`PrimitiveComponent.SetMassOverrideInKg` (`self.StaticMesh`) "None" 100.0 true)
  (set `/Game/ThirdPerson/Blueprints/BP_ThirdPersonCharacter.isGrabbingBox?` true (`self.Character Reference`)))

(fn `Release Box`
  (bind _physicsconstraint (`self.PhysicsConstraint`))
  (bind _character_default_max_walk_speed (`self.Character Default Max Walk Speed`))
  (bind _charactermovement (`Character.CharacterMovement` (`self.Character Reference`)))
  (bind _returnvalue (`PhysicsConstraintComponent.IsBroken` _physicsconstraint))
  (if (not _returnvalue)
    (`PhysicsConstraintComponent.BreakConstraint` _physicsconstraint))
  (`ActorComponent.Deactivate` (`self.PhysicsConstraint`))
  (set `CharacterMovementComponent.bOrientRotationToMovement` true _charactermovement)
  (if (> _character_default_max_walk_speed 0.0)
    (set `CharacterMovementComponent.MaxWalkSpeed` _character_default_max_walk_speed _charactermovement)
    (`PrimitiveComponent.SetMassOverrideInKg` (`self.StaticMesh`) "None" 5000.0 true)
    (set `/Game/ThirdPerson/Blueprints/BP_ThirdPersonCharacter.isGrabbingBox?` false (`self.Character Reference`))))

(fn `Set Player Grabbing Position`
  (bind _closestloc (`self.ClosestLoc`))
  (bind _returnvalue (`SceneComponent.K2_GetComponentLocation` _closestloc))
  (bind _returnvalue_2 (`SceneComponent.K2_GetComponentRotation` _closestloc))
  (bind (_returnvalue_x _returnvalue_y _returnvalue_z) (`KismetMathLibrary.BreakVector` (`SceneComponent.K2_GetComponentLocation` (`Character.CapsuleComponent` (`self.Character Reference`)))))
  (set `self.minDistance` 9999999.0)
  (for _array_element (`|MakeArray` (`self.PCLoc1`) (`self.PCLoc2`) (`self.PCLoc3`) (`self.PCLoc4`))
    (bind _returnvalue_3 (`KismetMathLibrary.Vector_Distance` (`SceneComponent.K2_GetComponentLocation` (`Character.CapsuleComponent` (`self.Character Reference`))) (`SceneComponent.K2_GetComponentLocation` _array_element)))
    (`/Engine/EditorBlueprintResources/StandardMacros.CompareFloat` _returnvalue_3 (`self.minDistance`)
      (:`<`
        (set `self.minDistance` _returnvalue_3)
        (set `self.ClosestLoc` _array_element))))
  (`SceneComponent.K2_SetWorldLocationAndRotation` (`self.PhysicsConstraint`) _returnvalue _returnvalue_2 false true)
  (`SceneComponent.K2_SetWorldLocationAndRotation` (`Character.CapsuleComponent` (`self.Character Reference`)) (`KismetMathLibrary.MakeVector` (.x _returnvalue) (.y _returnvalue) _returnvalue_z) _returnvalue_2 false true))

(fn `UserConstructionScript`
  (bind _quantumlightdetectorreference (`self.QuantumLightDetectorReference`))
  (bind (_boxextent_x _boxextent_y) (`KismetMathLibrary.BreakVector` (`BoxComponent.BoxExtent` (`self.Box`))))
  (bind _returnvalue (- _boxextent_y 25.0))
  (bind _returnvalue_2 (- _boxextent_x 25.0))
  (`SceneComponent.K2_SetRelativeLocation` (`self.PCLoc1`) (`KismetMathLibrary.MakeVector` (* _returnvalue_2 -1.0)) false true)
  (`SceneComponent.K2_SetRelativeLocation` (`self.PCLoc2`) (`KismetMathLibrary.MakeVector` _returnvalue_2) false true)
  (`SceneComponent.K2_SetRelativeLocation` (`self.PCLoc3`) (`KismetMathLibrary.MakeVector` 0.0 (* _returnvalue -1.0)) false true)
  (`SceneComponent.K2_SetRelativeLocation` (`self.PCLoc4`) (`KismetMathLibrary.MakeVector` 0.0 _returnvalue) false true)
  (`/Engine/EditorBlueprintResources/StandardMacros.IsValid` _quantumlightdetectorreference
    (:`Is Valid`
      (`self.K2_AttachToActor` _quantumlightdetectorreference self "None" "KeepWorld" "KeepWorld" "KeepWorld" true))))