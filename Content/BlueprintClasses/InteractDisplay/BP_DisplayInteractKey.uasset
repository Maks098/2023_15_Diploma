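; BP_DisplayInteractKey is an interact-key prompt that shows an animated Text3D letter.
; Show and Hide toggle the text's visibility and the LetterShown flag, with Show also resetting the animation phase.
; While shown, Tick advances a FloatSpeed-scaled timer that wraps over a symmetric range.
; Its absolute value drives a linear up-and-down bob and its signed value a continuous yaw spin, so the wrap is seamless.
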(event `self.ReceiveTick`
  (params (DeltaSeconds :type "Float (single-precision)"))
  (bind _text3d (`self.Text3D`))
  (bind (_relativelocation_x _relativelocation_y) (`KismetMathLibrary.BreakVector` (`SceneComponent.RelativeLocation` _text3d)))
  (bind (_relativerotation_roll _relativerotation_pitch) (`KismetMathLibrary.BreakRotator` (`SceneComponent.RelativeRotation` _text3d)))
  (if (`self.LetterShown`)
    (bind _output_get (set `self.CummTime` (+ (* DeltaSeconds (`self.FloatSpeed`)) (`self.CummTime`))))
    (if (>= _output_get 2.0)
      (set `self.CummTime` -2.0))
    (`SceneComponent.K2_SetRelativeLocationAndRotation` _text3d (`KismetMathLibrary.MakeVector` _relativelocation_x _relativelocation_y (* (`KismetMathLibrary.Abs` (`self.CummTime`)) 10.0)) (`KismetMathLibrary.MakeRotator` _relativerotation_roll _relativerotation_pitch (* (`self.CummTime`) 90.0)) false false)))

(event `Show`
  (`SceneComponent.SetHiddenInGame` (`self.Text3D`) false false)
  (set `self.LetterShown` true)
  (set `self.CummTime` -1.5))

(event `Hide`
  (`SceneComponent.SetHiddenInGame` (`self.Text3D`) true false)
  (set `self.LetterShown` false))

(fn `UserConstructionScript`)