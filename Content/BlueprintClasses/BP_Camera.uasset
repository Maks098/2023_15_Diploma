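; BP_Camera is the main menu camera, which becomes the view target on play, shows the cursor and creates the MainMenu widget.
; The widget triggers MoveCamera, which pushes a sound mix fading out master volume while timelines rotate the root and move the CineCamera in chained stages.
; A white fade-out sequence plays during the final inward move, after which it hides the cursor and opens the CutsceneAfterMainMenu level.
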(event `self.ReceiveBeginPlay`
  (bind _returnvalue (`GameplayStatics.GetPlayerController` 0))
  (set `self.bFindCameraComponentWhenViewTarget` true)
  (set `PlayerController.bShowMouseCursor` true _returnvalue)
  (`PlayerController.SetViewTargetWithBlend` _returnvalue self 0.0 "VTBlend_Cubic" 0.0 false)
  (bind _returnvalue_2 (`|CreateWidget` "/Game/Widgets/MainMenu_Widget.MainMenu_Widget_C"))
  (`UserWidget.AddToViewport` _returnvalue_2 0)
  (add `/Game/Widgets/MainMenu_Widget.MoveCamera` _returnvalue_2 (delegate `MoveCamera`)))

(event `MoveCamera`
  (`GameplayStatics.SetSoundMixClassOverride` "/Game/Audio/MasterClassMix.MasterClassMix" "/Engine/EngineSounds/Master.Master" 0.0 1.0 3.5)
  (`GameplayStatics.PushSoundMixModifier` "/Game/Audio/MasterClassMix.MasterClassMix")
  (`|ExecutionSequence`
    (:`then_0`
      (bind (_direction _y _z _x) (`Timeline|TimelineLocation`)
        (:`Update`
          (`SceneComponent.K2_SetRelativeLocation` (`self.CineCamera`) (`KismetMathLibrary.MakeVector` _x _y _z) true false))
        (:`Finished`
          (bind (_direction_2 _newtrack_0) (`Timeline|TimelineLocationBackwards`)
            (:`Update`
              (`SceneComponent.K2_SetRelativeLocation` (`self.CineCamera`) (`KismetMathLibrary.MakeVector` _newtrack_0 -410.0 -50.0) true false))
            (:`Finished`
              (bind _outactor (`LevelSequencePlayer.CreateLevelSequencePlayer` "/Game/BlueprintClasses/Dialogue/FadeOutWhite.FadeOutWhite"))
              (`MovieSceneSequencePlayer.Play` (`LevelSequenceActor.SequencePlayer` _outactor))
              (bind (_direction_3 _newtrack_0_2) (`Timeline|TimelineInwards`)
                (:`Update`
                  (`SceneComponent.K2_SetRelativeLocation` (`self.CineCamera`) (`KismetMathLibrary.MakeVector` _newtrack_0_2 -410.0 -50.0) true false))
                (:`Finished`
                  (set `PlayerController.bShowMouseCursor` false (`GameplayStatics.GetPlayerController` 0))
                  (`GameplayStatics.OpenLevel` "CutsceneAfterMainMenu"))))))))
    (:`then_1`
      (bind (_direction_4 _y_2 _z_2) (`Timeline|Timeline`)
        (:`Update`
          (`SceneComponent.K2_SetWorldRotation` (`self.DefaultSceneRoot`) (`KismetMathLibrary.MakeRotator` 0.0 _y_2 _z_2) false false))))))

(fn `MoveThatCamera`)

(fn `UserConstructionScript`)