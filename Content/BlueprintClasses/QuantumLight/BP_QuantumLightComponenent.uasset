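; Quantum light source that projects a cone of light, notifying QuantumLightDetectors it hits and pairing with other light sources, which act as blockers.
; A looping timer sweeps multi-line traces across yaw and pitch, and detectors behind a blocker are skipped.
; Pairing stores ID and distance on both lights, and expires through a timer reset on blocker hits.
; Edge traces of the first pitch row resize the two side panels bounding the cone.
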(event `self.ReceiveBeginPlay`
  (`self.EnableInput` (`GameplayStatics.GetPlayerController` 0))
  (`KismetSystemLibrary.K2_SetTimer` null "Create 3D Cone" (/ 1.0 (`self.UpdateFrequency`)) true))

(fn `Create 2D Cone`
  (params (`Y (Pitch)` :type "Float (single-precision)") (IsFIrtstIn :type Boolean))
  (locals (Index :type Integer))
  (bind _returnvalue (`self.K2_GetActorLocation`))
  (bind _index (`local.Index`))
  (bind _isfirtstin (`local.IsFIrtstIn`))
  (for _index_2 (range (+ (`self.NumOfTracesYaw`) 1))
    (set `local.Index` _index_2)
    (bind _outhits (`KismetSystemLibrary.LineTraceMulti` :`Start` _returnvalue :`End` (+ _returnvalue (* (`self.LineLength`) (`KismetMathLibrary.RotateAngleAxis` (`KismetMathLibrary.GreaterGreater_VectorRotator` (`KismetMathLibrary.CreateVectorFromYawPitch` (* (`KismetMathLibrary.Conv_IntToDouble` (`self.AngleRangeYaw`)) -0.5) (* (/ (`KismetMathLibrary.Conv_IntToDouble` (`self.AngleRangePitch`)) (`KismetMathLibrary.Conv_IntToDouble` (`self.NumOfTracesPitch`))) `Y (Pitch)` -1.0)) (`self.K2_GetActorRotation`)) (* (`KismetMathLibrary.Conv_IntToDouble` _index_2) (/ (`KismetMathLibrary.Conv_IntToDouble` (`self.AngleRangeYaw`)) (`KismetMathLibrary.Conv_IntToDouble` (`self.NumOfTracesYaw`)))) (0.0 0.0 1.0)))) :`TraceChannel` "TraceTypeQuery3" :`DrawDebugType` "ForDuration" :`DrawTime` (/ 1.0 (`self.UpdateFrequency`))))
    (`self.Process Hits in Once Trace` _outhits (and (== _index 0) _isfirtstin) (and _isfirtstin (== _index (`self.NumOfTracesYaw`))))))

(fn `Create 3D Cone`
  (bind (_firsthitidlight _hitpanelsleft _hitpanelsright) (break `/Game/DataTypes/Structs/DataForPanelsInTrace` (`self.DataForPanels`)))
  (bind _returnvalue (`KismetArrayLibrary.Array_LastIndex` _hitpanelsleft))
  (bind _returnvalue_2 (`KismetArrayLibrary.Array_LastIndex` _hitpanelsright))
  (set `self.DataForPanels` (make `/Game/DataTypes/Structs/DataForPanelsInTrace` -1))
  (for _index (range (+ (`self.NumOfTracesPitch`) 1))
    (bind _returnvalue_3 (== _index 0))
    (`self.Create 2D Cone` (`KismetMathLibrary.Conv_IntToDouble` _index) _returnvalue_3)
    (if _returnvalue_3
      (if (not (or (or (== _firsthitidlight -1) (== _returnvalue -1)) (== _returnvalue_2 -1)))
        (`self.ScalePanelsToUnits` (`|GetArrayItem` _hitpanelsleft _returnvalue) (`|GetArrayItem` _hitpanelsright _returnvalue_2))))))

(fn `Process Hits in Once Trace`
  (params (HitOuts :type "Array of HitResult Structure") (IsLeftIn :type Boolean) (IsRightIn :type Boolean))
  (locals (HasHitBlocker :type Boolean) (HitBlocker :type "/Game/BlueprintClasses/QuantumLight/BP_QuantumLightComponenent Object Reference"))
  (bind (_firsthitidlight _hitpanelsleft _hitpanelsright) (break `/Game/DataTypes/Structs/DataForPanelsInTrace` (`self.DataForPanels`)))
  (bind (_firsthitidlight_2 _hitpanelsleft_2 _hitpanelsright_2) (break `/Game/DataTypes/Structs/DataForPanelsInTrace` (`self.DataForPanels`)))
  (set `local.HasHitBlocker` false)
  (for _array_element HitOuts
    (bind (_bblockinghit _binitialoverlap _time _distance _location _impactpoint _normal _impactnormal _physmat _hitactor) (`GameplayStatics.BreakHitResult` _array_element))
    ;[1 1 1] HitQuantumLigthBlocker
    (bind _asbp_quantum_light_componenent (cast `/Game/BlueprintClasses/QuantumLight/BP_QuantumLightComponenent` _hitactor)
      (:`then`
        (`|ExecutionSequence`
          (:`then_0`
            (bind _hashitblockerout (`self.ProcessIfBlocker` _asbp_quantum_light_componenent _distance (`local.HasHitBlocker`)))
            (if (not (`local.HasHitBlocker`))
              (set `local.HasHitBlocker` _hashitblockerout)))
          (:`then_1`
            (if (or (`local.IsLeftIn`) (`local.IsRightIn`))
              (if (== _firsthitidlight -1)
                (bind _idlightsource (`/Game/BlueprintClasses/QuantumLight/BP_QuantumLightComponenent.IdLightSource` _asbp_quantum_light_componenent))
                (set `self.DataForPanels` (make `/Game/DataTypes/Structs/DataForPanelsInTrace` _idlightsource _hitpanelsleft _hitpanelsright)))
              (if (== _idlightsource _firsthitidlight)
                (if (`local.IsLeftIn`)
                  (bind _returnvalue (+ _distance 1.0))
                  (`KismetArrayLibrary.Array_Add` _hitpanelsleft_2 _returnvalue)
                  (elif (`local.IsRightIn`)
                    (`KismetArrayLibrary.Array_Add` _hitpanelsright_2 _returnvalue))))))))
      (:`CastFailed`
        ;[1 1 1] HitQuantumDetector
        (bind _asquantum_light_detector (cast `/Game/BlueprintClasses/QuantumLightDetector` _hitactor))
        (if (not (`local.HasHitBlocker`))
          (`/Game/BlueprintClasses/QuantumLightDetector.HitWithQuantumLight` _asquantum_light_detector))))))

(fn `ProcessIfBlocker`
  (params (HitLight :type "/Game/BlueprintClasses/QuantumLight/BP_QuantumLightComponenent Object Reference") (Distance :type "Float (double-precision)") (HasHitBlockerIn :type Boolean))
  (returns (HasHitBlockerOut :type Boolean))
  (locals (HitPairedId :type Integer) (HitPairdedDistance :type "Float (double-precision)") (HitId :type Integer :default 0) (MyPairedId :type Integer) (MyPairedDistance :type "Float (double-precision)") (DistanceToHit :type "Float (double-precision)") (HasHitBlocker :type Boolean))
  (bind (_idpairedlight _distance) (break `/Game/DataTypes/Structs/TraceDataStruct` (`/Game/BlueprintClasses/QuantumLight/BP_QuantumLightComponenent.PairedQuantum` HitLight)))
  (bind (_idpairedlight_2 _distance_2) (break `/Game/DataTypes/Structs/TraceDataStruct` (`self.PairedQuantum`)))
  (`|ExecutionSequence`
    (:`then_0`
      (set `local.HitPairedId` _idpairedlight)
      (set `local.HitPairdedDistance` _distance)
      (set `local.HitId` (`/Game/BlueprintClasses/QuantumLight/BP_QuantumLightComponenent.IdLightSource` HitLight))
      (set `local.MyPairedId` _idpairedlight_2)
      (set `local.MyPairedDistance` _distance_2)
      (set `local.DistanceToHit` Distance)
      (set `local.HasHitBlocker` HasHitBlockerIn))
    (:`then_1`
      (if (and (== (`local.HitPairedId`) -1) (== (`local.MyPairedId`) -1))
        (`self.ProcessBlockerSetIds`
          (:`OutputPin`
            (set `local.HasHitBlocker` true :!label _label)
            (`self.ResetUnpairTimer`)
            (set `self.PairedQuantum` (make `/Game/DataTypes/Structs/TraceDataStruct` (`local.MyPairedId`) (`local.MyPairedDistance`)))
            (set `/Game/BlueprintClasses/QuantumLight/BP_QuantumLightComponenent.PairedQuantum` (make `/Game/DataTypes/Structs/TraceDataStruct` (`local.HitPairedId`) (`local.HitPairdedDistance`)) HitLight)
            (return (`local.HasHitBlocker`))))
        (elif (== (`local.MyPairedId`) -1)
          (`|ExecutionSequence`)
          (elif (== (`local.HitPairedId`) (`self.IdLightSource`))
            (if (!= (`local.DistanceToHit`) (`local.MyPairedDistance`))
              (set `local.MyPairedDistance` (`local.DistanceToHit`))
              (goto _label)
              (else
                (goto _label)))
            (elif (< (`local.DistanceToHit`) (`local.MyPairedDistance`))
              (`self.ProcessBlockerSetIds`
                (:`OutputPin`
                  (goto _label))))))))))

(fn `ResetUnpairTimer`
  (bind _unpairtimer (`self.UnpairTimer`))
  (if (`KismetSystemLibrary.K2_IsValidTimerHandle` _unpairtimer)
    (`KismetSystemLibrary.K2_ClearAndInvalidateTimerHandle` _unpairtimer))
  (bind _returnvalue (`KismetSystemLibrary.K2_SetTimer` null "Unpair" (/ 1.0 (`self.UpdateFrequency`)) false 0.01))
  (set `self.UnpairTimer` _returnvalue))

(fn `ScalePanelsToUnits`
  (params (LineLengthLeft :type "Float (double-precision)") (NewParamRight :type "Float (double-precision)"))
  (bind _lewy_panel (`self.Lewy panel`))
  (bind _prawy_panel (`self.Prawy panel`))
  (bind (_relativescale3d_x _relativescale3d_y _relativescale3d_z) (`KismetMathLibrary.BreakVector` (`SceneComponent.RelativeScale3D` _prawy_panel)))
  (bind (_relativescale3d_x_2 _relativescale3d_y_2 _relativescale3d_z_2) (`KismetMathLibrary.BreakVector` (`SceneComponent.RelativeScale3D` _lewy_panel)))
  ;[1 1 1] Set Scale of Planes
  (`|ExecutionSequence`
    (:`then_0`
      (`SceneComponent.SetRelativeScale3D` _lewy_panel (`KismetMathLibrary.MakeVector` (/ LineLengthLeft 100.0) _relativescale3d_y_2 _relativescale3d_z_2))
      ;[1 1 1] Set Location of Planes
      (`SceneComponent.K2_SetRelativeLocation` _lewy_panel (`KismetMathLibrary.MakeVector` (/ LineLengthLeft 2.0)) false false))
    (:`then_1`
      (`SceneComponent.SetRelativeScale3D` _prawy_panel (`KismetMathLibrary.MakeVector` (/ NewParamRight 100.0) _relativescale3d_y _relativescale3d_z))
      (`SceneComponent.K2_SetRelativeLocation` _prawy_panel (`KismetMathLibrary.MakeVector` (/ NewParamRight 2.0)) false false))))

(fn `Unpair`
  (bind _linelength (`self.LineLength`))
  (set `self.PairedQuantum` (make `/Game/DataTypes/Structs/TraceDataStruct` -1))
  (set `self.DataForPanels` (make `/Game/DataTypes/Structs/DataForPanelsInTrace` -1))
  (`self.ScalePanelsToUnits` _linelength _linelength)
  (`KismetSystemLibrary.PrintString` (`KismetStringLibrary.Concat_StrStr` "Id: " (`KismetStringLibrary.Conv_IntToString` (`self.IdLightSource`)) "Unpaired")))

(fn `UserConstructionScript`
  (bind _linelength (`self.LineLength`))
  (bind _returnvalue (`KismetMathLibrary.Conv_IntToDouble` (`self.AngleRangeYaw`)))
  (`|ExecutionSequence`
    (:`then_0`
      ;[1 1 1] Set Yaw of planes / scenes
      (`|ExecutionSequence`
        (:`then_0`
          (`SceneComponent.K2_SetRelativeRotation` (`self.Lewa scena`) (`KismetMathLibrary.MakeRotator` 0.0 0.0 (* _returnvalue -0.5)) false false))
        (:`then_1`
          (`SceneComponent.K2_SetRelativeRotation` (`self.Prawa scena`) (`KismetMathLibrary.MakeRotator` 0.0 0.0 (* _returnvalue 0.5)) false false))))
    (:`then_1`
      (`self.ScalePanelsToUnits` _linelength _linelength))))