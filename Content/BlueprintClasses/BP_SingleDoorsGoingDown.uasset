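; A single sliding door that moves vertically and streams levels in and out as it changes state.
; A Timeline's alpha drives the door mesh's relative Z position, and the door plays it on BeginPlay if it starts switched on.
; Turnon loads a named stream level without blocking and plays the Timeline, while TurnOff unloads another named level and reverses it.
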(event `self.ReceiveBeginPlay`
  (`self.EnableInput` (`GameplayStatics.GetPlayerController` 0))
  (if (`self.IsOn`)
    (bind (_direction _alpha) (`Timeline|Timeline` :!label _label)
      (:`Update`
        (`SceneComponent.K2_SetRelativeLocation` (`self.Door_Single_Door_Single`) (`KismetMathLibrary.MakeVector` 0.0 -100.0 _alpha) false false)))))

(event `self.TurnOn`
  (`GameplayStatics.LoadStreamLevel` (`KismetStringLibrary.Conv_StringToName` (`self.LevelToLoad`)) true)
  (goto _label))

(event `self.TurnOff`
  (`GameplayStatics.UnloadStreamLevel` (`KismetStringLibrary.Conv_StringToName` (`self.LevelToUnload`)))
  (goto _label :!via `Reverse`))

(fn `UserConstructionScript`)