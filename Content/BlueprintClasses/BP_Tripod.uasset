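; BP_Tripod is an interactable tripod that holds the item carried by BP_ThirdPersonCharacter, using a socket named FlashlightSocket.
; Its box overlap enables input while the character is inside and disables it on exit.
; Pressing E drives a FlipFlop that alternately snaps the held item onto the tripod and back onto the character's mesh, swapping the HeldItem and PlacedItem references.
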(event `Key|E`
  (params (Key :type "Key Structure"))
  (bind _placeditem (`self.PlacedItem`))
  (:`Pressed`
    (bind _asbp_third_person_character (cast `/Game/ThirdPerson/Blueprints/BP_ThirdPersonCharacter` (stale `self.Box.OnComponentBeginOverlap` OtherActor)))
    (`/Engine/EditorBlueprintResources/StandardMacros.FlipFlop`
      (:`A`
        (bind _helditem (`/Game/ThirdPerson/Blueprints/BP_ThirdPersonCharacter.HeldItem` _asbp_third_person_character))
        (`self.K2_AttachToComponent` _helditem (`self.Tripod`) "FlashlightSocket" "SnapToTarget" "SnapToTarget" "KeepWorld" true)
        (set `self.PlacedItem` _helditem)
        (set `/Game/ThirdPerson/Blueprints/BP_ThirdPersonCharacter.HeldItem` null _asbp_third_person_character))
      (:`B`
        (`self.K2_AttachToComponent` _placeditem (`Character.Mesh` _asbp_third_person_character) "FlashlightSocket" "SnapToTarget" "SnapToTarget" "KeepWorld" true)
        (set `/Game/ThirdPerson/Blueprints/BP_ThirdPersonCharacter.HeldItem` _placeditem _asbp_third_person_character)
        (set `self.PlacedItem` null)))))

(event `self.Box.OnComponentBeginOverlap`
  (params (OverlappedComponent :type "PrimitiveComponent Object Reference") (OtherActor :type "Actor Object Reference") (OtherComp :type "PrimitiveComponent Object Reference") (OtherBodyIndex :type Integer) (bFromSweep :type Boolean) (SweepResult :type "HitResult Structure (by ref)"))
  (cast `/Game/ThirdPerson/Blueprints/BP_ThirdPersonCharacter` OtherActor)
  (`self.EnableInput` (`GameplayStatics.GetPlayerController` 0)))

(event `self.Box.OnComponentEndOverlap`
  (params (OverlappedComponent :type "PrimitiveComponent Object Reference") (OtherActor :type "Actor Object Reference") (OtherComp :type "PrimitiveComponent Object Reference") (OtherBodyIndex :type Integer))
  (cast `/Game/ThirdPerson/Blueprints/BP_ThirdPersonCharacter` OtherActor)
  (`self.DisableInput` (`GameplayStatics.GetPlayerController` 0)))

(fn `UserConstructionScript`)