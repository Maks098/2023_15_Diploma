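; BP_AndNode is an AND gate logic component that switches a referenced interactable on only while all its inputs are on.
; The construction script creates a configurable number of signal slots and evenly spaced input diode child actors.
; Turnon fills the first off slot and TurnOff clears the last on one, so inputs are anonymous.
; UpdateOutput then toggles the interactable and output diode only when the combined state changes.
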(event `self.ReceiveBeginPlay`
  (bind _asbp_diode (cast `/Game/BlueprintClasses/Diode/BP_Diode` (`ChildActorComponent.ChildActor` (`self.DiodeOut`))))
  (set `self.DiodeBPOut` _asbp_diode))

(event `/Game/BlueprintClasses/OnOffInterface.TurnOff`
  (bind _connectedsignals (`self.ConnectedSignals`))
  (bind _returnvalue (`KismetArrayLibrary.Array_Length` _connectedsignals))
  (for _index (range (+ _returnvalue 1))
    (bind _returnvalue_2 (- (- _returnvalue 1) _index))
    (if (`|GetArrayItem` _connectedsignals _returnvalue_2)
      (`KismetArrayLibrary.Array_Set` _connectedsignals _returnvalue_2)
      (`/Game/BlueprintClasses/OnOffInterface.TurnOff` (`|GetArrayItem` (`self.DiodesIn`) _returnvalue_2))
      (`self.Update Output`)
      (break))))

(event `/Game/BlueprintClasses/OnOffInterface.TurnOn`
  (bind _connectedsignals (`self.ConnectedSignals`))
  (for (_array_element _array_index) _connectedsignals
    (if (not _array_element)
      (`KismetArrayLibrary.Array_Set` _connectedsignals _array_index true)
      (`/Game/BlueprintClasses/OnOffInterface.TurnOn` (`|GetArrayItem` (`self.DiodesIn`) _array_index))
      (`self.Update Output`)
      (break))))

(fn `Update Output`
  (locals (AnyOffFlag :type Boolean))
  (bind _diodebpout (`self.DiodeBPOut`))
  (bind _interactable_reference (`self.Interactable Reference`))
  (bind _state (`self.State`))
  (set `local.AnyOffFlag` false)
  (for _array_element (`self.ConnectedSignals`)
    (if (not _array_element)
      (set `local.AnyOffFlag` true)
      (break)))
  (if (`local.AnyOffFlag`)
    (if _state
      (`/Game/BlueprintClasses/OnOffInterface.TurnOff` _interactable_reference)
      (`/Game/BlueprintClasses/OnOffInterface.TurnOff` _diodebpout)
      (set `self.State` (not (`self.State`)) :!label _label))
    (elif (not _state)
      (`/Game/BlueprintClasses/OnOffInterface.TurnOn` _interactable_reference)
      (`/Game/BlueprintClasses/OnOffInterface.TurnOn` _diodebpout)
      (goto _label))))

(fn `UserConstructionScript`
  (locals (UppedDiodeSpace :type "Float (double-precision)" :default 100.0))
  (bind _returnvalue (- (`self.HowManyConnnected`) 1))
  (`|ExecutionSequence`
    (:`then_0`
      (for _ (range (`self.HowManyConnnected`))
        (`KismetArrayLibrary.Array_Add` (`self.ConnectedSignals`))))
    (:`then_1`
      (for _index (range (+ _returnvalue 1))
        (bind _returnvalue_2 (`AddComponent|NODE_AddChildActorComponent-1` :`RelativeTransform` (`KismetMathLibrary.MakeTransform` (`KismetMathLibrary.MakeVector` (+ (/ (`local.UppedDiodeSpace`) -2.0) (* (`KismetMathLibrary.Conv_IntToDouble` (+ _index 1)) (/ (`local.UppedDiodeSpace`) (`KismetMathLibrary.Conv_IntToDouble` (+ _returnvalue 2))))) 9.0 25.0))))
        (bind _asbp_diode (cast `/Game/BlueprintClasses/Diode/BP_Diode` (`ChildActorComponent.ChildActor` _returnvalue_2)))
        (`KismetArrayLibrary.Array_Add` (`self.DiodesIn`) _asbp_diode)))))