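; BP_FlipFLopNode is a logic component that toggles a referenced interactable on and off, acting as an edge-triggered flip-flop.
; Turnon toggles the stored State only when RisingEdge is set, and TurnOff feeds the same toggle only when FallingEdge is set.
; Each toggle switches InteractableReference and the output BP_Diode together.
; BeginPlay caches the output diode from its child actor and lights indicator diodes for the enabled edges.
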(event `self.ReceiveBeginPlay`
  (`|ExecutionSequence`
    (:`then_0`
      (bind _asbp_diode (cast `/Game/BlueprintClasses/Diode/BP_Diode` (`ChildActorComponent.ChildActor` (`self.DiodeOut`))))
      (set `self.DiodeBPOut` _asbp_diode))
    (:`then_1`
      (if (`self.RisingEdge`)
        (bind _asbp_diode_2 (cast `/Game/BlueprintClasses/Diode/BP_Diode` (`ChildActorComponent.ChildActor` (`self.DiodeRising`))))
        (`/Game/BlueprintClasses/OnOffInterface.TurnOn` _asbp_diode_2)))
    (:`then_2`
      (if (`self.FallingEdge`)
        (bind _asbp_diode_3 (cast `/Game/BlueprintClasses/Diode/BP_Diode` (`ChildActorComponent.ChildActor` (`self.DiodeFaling`))))
        (`self.TurnOn` _asbp_diode_3)))))

(event `/Game/BlueprintClasses/OnOffInterface.TurnOn`
  (bind _diodebpout (`self.DiodeBPOut`))
  (bind _interactable_reference (`self.Interactable Reference`))
  (if (`self.RisingEdge`)
    (if (`self.State`) :!label _label
      (`/Game/BlueprintClasses/OnOffInterface.TurnOff` _interactable_reference)
      (`/Game/BlueprintClasses/OnOffInterface.TurnOff` _diodebpout)
      (else
        (`/Game/BlueprintClasses/OnOffInterface.TurnOn` _interactable_reference)
        (`self.TurnOn` _diodebpout)))
    (set `self.State` (not (`self.State`)))))

(event `/Game/BlueprintClasses/OnOffInterface.TurnOff`
  (if (`self.FallingEdge`)
    (goto _label)))

(fn `UserConstructionScript`)