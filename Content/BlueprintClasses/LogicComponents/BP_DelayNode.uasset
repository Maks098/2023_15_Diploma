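; BP_DelayNode is a logic component that forwards TurnOn and TurnOff signals to a referenced interactable after separate configurable delays.
; Each signal switches the input diode at once and restarts its named timer, which later switches the interactable and output diode.
; A new signal cancels the opposite pending timer only when its own delay is shorter or equal, so otherwise both changes still fire.
; Both diodes are child actors cast to BP_Diode on BeginPlay.
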(event `self.ReceiveBeginPlay`
  (`|ExecutionSequence`
    (:`then_0`
      (bind _asbp_diode (cast `/Game/BlueprintClasses/Diode/BP_Diode` (`ChildActorComponent.ChildActor` (`self.DiodeOut`))))
      (set `self.DiodeBPOut` _asbp_diode))
    (:`then_1`
      (bind _asbp_diode_2 (cast `/Game/BlueprintClasses/Diode/BP_Diode` (`ChildActorComponent.ChildActor` (`self.DiodeIn`))))
      (set `self.DiodeBPIn` _asbp_diode_2))))

(event `/Game/BlueprintClasses/OnOffInterface.TurnOn`
  (bind _ondelayhandle (`self.OnDelayHandle`))
  (`/Game/BlueprintClasses/OnOffInterface.TurnOn` (`self.DiodeBPIn`))
  (if (`KismetSystemLibrary.K2_IsValidTimerHandle` _ondelayhandle)
    (`KismetSystemLibrary.K2_ClearAndInvalidateTimerHandle` _ondelayhandle))
  (bind _returnvalue (`KismetSystemLibrary.K2_SetTimer` null "OnDelay" (+ (`self.TurnOnDelay`) 1e-06)))
  (bind _output_get (set `self.OnDelayHandle` _returnvalue))
  (if (and (<= (`self.TurnOnDelay`) (`self.TurnOffDelay`)) (`KismetSystemLibrary.K2_IsValidTimerHandle` (stale `/Game/BlueprintClasses/OnOffInterface.TurnOff` _output_get)))
    (`KismetSystemLibrary.K2_ClearAndInvalidateTimerHandle` (stale `/Game/BlueprintClasses/OnOffInterface.TurnOff` _output_get))))

(event `/Game/BlueprintClasses/OnOffInterface.TurnOff`
  (bind _offdelayhandle (`self.OffDelayHandle`))
  (`/Game/BlueprintClasses/OnOffInterface.TurnOff` (`self.DiodeBPIn`))
  (if (`KismetSystemLibrary.K2_IsValidTimerHandle` _offdelayhandle)
    (`KismetSystemLibrary.K2_ClearAndInvalidateTimerHandle` _offdelayhandle))
  (bind _returnvalue (`KismetSystemLibrary.K2_SetTimer` null "OffDelay" (+ (`self.TurnOffDelay`) 1e-06)))
  (bind _output_get (set `self.OffDelayHandle` _returnvalue))
  (if (and (<= (`self.TurnOffDelay`) (`self.TurnOnDelay`)) (`KismetSystemLibrary.K2_IsValidTimerHandle` (`self.OnDelayHandle`)))
    (`KismetSystemLibrary.K2_ClearAndInvalidateTimerHandle` (stale `/Game/BlueprintClasses/OnOffInterface.TurnOn` _output_get))))

(fn `OffDelay`
  (`/Game/BlueprintClasses/OnOffInterface.TurnOff` (`self.Interactable Reference`))
  (`KismetSystemLibrary.K2_InvalidateTimerHandle` (`self.OffDelayHandle`))
  (`/Game/BlueprintClasses/OnOffInterface.TurnOff` (`self.DiodeBPOut`)))

(fn `OnDelay`
  (`/Game/BlueprintClasses/OnOffInterface.TurnOn` (`self.Interactable Reference`))
  (`KismetSystemLibrary.K2_InvalidateTimerHandle` (`self.OnDelayHandle`))
  (`/Game/BlueprintClasses/OnOffInterface.TurnOn` (`self.DiodeBPOut`)))

(fn `UserConstructionScript`)