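; BP_NotNode is a logic component that inverts an on/off signal for a referenced interactable.
; Its Turnon event switches the interactable off, and TurnOff switches it on.
; UpdateDiode stores the input state and lights input and output diodes, cast from child actors on BeginPlay, in opposite states.
; StartWIthSignal makes BeginPlay run the TurnOff logic, so the output starts on.
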(event `/Game/BlueprintClasses/OnOffInterface.TurnOn`
  (`/Game/BlueprintClasses/OnOffInterface.TurnOff` (`self.Interactable Reference`))
  (`self.UpdateDiode` true))

(event `/Game/BlueprintClasses/OnOffInterface.TurnOff`
  (`self.TurnOn` (`self.Interactable Reference`) :!label _label)
  (`self.UpdateDiode` false))

(event `self.ReceiveBeginPlay`
  (`|ExecutionSequence`
    (:`then_0`
      (`|ExecutionSequence`
        (:`then_0`
          (bind _asbp_diode (cast `/Game/BlueprintClasses/Diode/BP_Diode` (`ChildActorComponent.ChildActor` (`self.DiodeIn`))))
          (set `self.DiodeBPIn` _asbp_diode))
        (:`then_1`
          (bind _asbp_diode_2 (cast `/Game/BlueprintClasses/Diode/BP_Diode` (`ChildActorComponent.ChildActor` (`self.DiodeOut`))))
          (set `self.DiodeBPOut` _asbp_diode_2))))
    (:`then_1`
      (if (`self.StartWIthSignal`)
        (goto _label)))))

(fn `UpdateDiode`
  (params (`On -1 / Off - 0` :type Boolean))
  (locals (OnOff :type Boolean))
  (bind _diodebpin (`self.DiodeBPIn`))
  (bind _diodebpout (`self.DiodeBPOut`))
  (set `local.OnOff` `On -1 / Off - 0`)
  (`|ExecutionSequence`
    (:`then_0`
      (if (`local.OnOff`)
        (`/Game/BlueprintClasses/OnOffInterface.TurnOn` _diodebpin)
        (else
          (`/Game/BlueprintClasses/OnOffInterface.TurnOff` _diodebpin))))
    (:`then_1`
      (if (`local.OnOff`)
        (`/Game/BlueprintClasses/OnOffInterface.TurnOff` _diodebpout)
        (else
          (`/Game/BlueprintClasses/OnOffInterface.TurnOn` _diodebpout))))))

(fn `UserConstructionScript`)