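; Switchable horizontal fan that pushes the player and ungrabbed BP_OldBox actors along one of four axis directions.
; Construction script derives rotation and push direction from FanOrientation, and sizes the trigger box and particle lifetime from FlowLength.
; Overlaps track targets; while on, async physics tick offsets their locations until the flow's end, adding velocity for boxes.
; TurnOn/TurnOff toggle particles and core material; SetPlayerBehaviour is empty and timer-driven movement is unused.
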(event `self.ReceiveBeginPlay`
  (bind _niagara (`self.Niagara`))
  (bind _base (`self.Base`))
  (`|ExecutionSequence`
    (:`then_0`
      (if (`self.IsOn`)
        ;[1 1 1] Animaiton
        (`FXSystemComponent.SetFloatParameter` _niagara "SpawnRate" 1.0 :!label _label)
        (`PrimitiveComponent.SetMaterial` _base 3 "/Game/BlenderFiles/Materials/Detector/OnCoreBlue.OnCoreBlue")
        (else
          (`KismetSystemLibrary.K2_PauseTimerHandle` (`self.MoveObjectsTimerHandle`))
          (`FXSystemComponent.SetFloatParameter` _niagara "SpawnRate" 0.0 :!label _label_2)
          (`PrimitiveComponent.SetMaterial` _base 3 "/Game/BlenderFiles/Materials/Detector/OffCoreBlue.OffCoreBlue"))))
    (:`then_1`
      (`KismetSystemLibrary.DelayUntilNextTick`)
      (for _array_element (`PrimitiveComponent.GetOverlappingActors` (`self.Box`) "/Game/BlueprintClasses/BP_OldBox.BP_OldBox_C")
        (bind _asbp_old_box (cast `/Game/BlueprintClasses/BP_OldBox` _array_element))
        (if (`PrimitiveComponent.IsOverlappingComponent` (`self.Box`) (`/Game/BlueprintClasses/BP_OldBox.StaticMesh` _asbp_old_box))
          (`KismetArrayLibrary.Array_AddUnique` (`self.Boxes`) _asbp_old_box))))))

(event `/Game/BlueprintClasses/OnOffInterface.TurnOn`
  ;[1 1 1] Animaiton
  (set `self.IsOn` true)
  (`self.TurnedOn`)
  (goto _label))

(event `self.ReceiveAsyncPhysicsTick`
  (params (DeltaSeconds :type "Float (single-precision)") (SimSeconds :type "Float (single-precision)"))
  (if (`self.IsOn`)
    (`self.MoveObjectsToSide` DeltaSeconds)))

(event `/Game/BlueprintClasses/OnOffInterface.TurnOff`
  ;[1 1 1] Animaiton
  (set `self.IsOn` false)
  (`self.TurnedOff`)
  (goto _label_2))

(event `TurnedOn`
  (`self.SetPlayerBehaviour` true)
  (for _ (`self.Boxes`)
    _))

(event `TurnedOff`
  (`self.SetPlayerBehaviour` false)
  (for _ (`self.Boxes`)
    _))

(event `self.Box.OnComponentBeginOverlap`
  (params (OverlappedComponent :type "PrimitiveComponent Object Reference") (OtherActor :type "Actor Object Reference") (OtherComp :type "PrimitiveComponent Object Reference") (OtherBodyIndex :type Integer) (bFromSweep :type Boolean) (SweepResult :type "HitResult Structure (by ref)"))
  (bind _asbp_third_person_character (cast `/Game/ThirdPerson/Blueprints/BP_ThirdPersonCharacter` OtherActor)
    (:`then`
      (set `self.Player` _asbp_third_person_character))
    (:`CastFailed`
      (bind _asbp_old_box (cast `/Game/BlueprintClasses/BP_OldBox` OtherActor))
      (cast `StaticMeshComponent` OtherComp)
      (`KismetArrayLibrary.Array_AddUnique` (`self.Boxes`) _asbp_old_box))))

(event `self.Box.OnComponentEndOverlap`
  (params (OverlappedComponent :type "PrimitiveComponent Object Reference") (OtherActor :type "Actor Object Reference") (OtherComp :type "PrimitiveComponent Object Reference") (OtherBodyIndex :type Integer))
  (cast `/Game/ThirdPerson/Blueprints/BP_ThirdPersonCharacter` OtherActor
    (:`then`
      (`self.SetPlayerBehaviour` false)
      (set `self.Player` null))
    (:`CastFailed`
      (bind _asbp_old_box (cast `/Game/BlueprintClasses/BP_OldBox` OtherActor))
      (cast `StaticMeshComponent` OtherComp)
      (`KismetArrayLibrary.Array_RemoveItem` (`self.Boxes`) _asbp_old_box))))

(fn `MoveObjectsToSide`
  (params (DeltaTime :type "Float (double-precision)"))
  (bind _returnvalue_x (`KismetMathLibrary.BreakVector` (`self.GetActorScale3D`)))
  (bind _returnvalue_x_2 (`KismetMathLibrary.BreakVector` (`self.GetActorScale3D`)))
  (bind (_returnvalue_x_3 _returnvalue_y) (`KismetMathLibrary.BreakVector` (`self.K2_GetActorLocation`)))
  (bind (_returnvalue_x_4 _returnvalue_y_2) (`KismetMathLibrary.BreakVector` (`self.K2_GetActorLocation`)))
  (bind _player (`self.Player`))
  (bind _moverate (`self.MoveRate`))
  (bind (_movedirection_x _movedirection_y) (`KismetMathLibrary.BreakVector` (`self.MoveDirection`)))
  (bind _deltatime (`local.DeltaTime`))
  (bind _moverate_2 (`self.MoveRate`))
  (bind (_movedirection_x_2 _movedirection_y_2) (`KismetMathLibrary.BreakVector` (`self.MoveDirection`)))
  (bind (_returnvalue_x_5 _returnvalue_y_3) (`KismetMathLibrary.BreakVector` (`self.K2_GetActorLocation` _player)))
  (bind (_returnvalue_x_6 _returnvalue_y_4 _returnvalue_z) (`KismetMathLibrary.BreakVector` (`self.K2_GetActorLocation` _player)))
  (bind _returnvalue (* (`self.FlowLength`) _returnvalue_x))
  (bind _returnvalue_2 (* (`self.FlowLength`) _returnvalue_x_2))
  (set `self.MoveRate` (* DeltaTime (`self.HowManyUnitsPerSecond`)))
  (`|ExecutionSequence`
    (:`then_0`
      (if (`KismetSystemLibrary.IsValid` _player)
        (switch `/Game/BlueprintClasses/Fans/FanOrientation` (`self.FanOrientation`)
          (:`NewEnumerator0`
            (if (<= _returnvalue_x_5 (+ _returnvalue_x_4 _returnvalue))
              (`self.K2_SetActorLocation` _player (`KismetMathLibrary.MakeVector` (+ _returnvalue_x_6 (* _moverate _movedirection_x)) (+ _returnvalue_y_4 (* _movedirection_y _moverate)) _returnvalue_z) false false :!label _label)))
          (:`NewEnumerator1`
            (if (<= _returnvalue_y_3 (+ _returnvalue_y_2 _returnvalue))
              (goto _label)))
          (:`NewEnumerator2`
            (if (>= _returnvalue_x_5 (- _returnvalue_x_4 _returnvalue))
              (goto _label)))
          (:`NewEnumerator3`
            (if (>= _returnvalue_y_3 (- _returnvalue_y_2 _returnvalue))
              (goto _label))))))
    (:`then_1`
      (for _array_element (`self.Boxes`)
        (if (`KismetSystemLibrary.IsValid` _array_element)
          (if (not (`/Game/BlueprintClasses/BP_OldBox.isBoxGrabbed?` _array_element))
            (switch `/Game/BlueprintClasses/Fans/FanOrientation` (`self.FanOrientation`)
              (:`NewEnumerator0`
                (bind (_returnvalue_x_7 _returnvalue_y_5) (`KismetMathLibrary.BreakVector` (`self.K2_GetActorLocation` _array_element)))
                (if (<= _returnvalue_x_7 (+ _returnvalue_x_3 _returnvalue_2 -50.0))
                  (bind (_returnvalue_x_8 _returnvalue_y_6 _returnvalue_z_2) (`KismetMathLibrary.BreakVector` (`self.K2_GetActorLocation` _array_element)))
                  (bind (_returnvalue_x_9 _returnvalue_y_7 _returnvalue_z_3) (`KismetMathLibrary.BreakVector` (`self.GetVelocity` _array_element)))
                  (`self.K2_SetActorLocation` _array_element (`KismetMathLibrary.MakeVector` (+ _returnvalue_x_8 (* _moverate_2 _movedirection_x_2) (* _deltatime _returnvalue_x_9)) (+ _returnvalue_y_6 (* _movedirection_y_2 _moverate_2) (* _deltatime _returnvalue_y_7)) (+ _returnvalue_z_2 (* _deltatime _returnvalue_z_3 0.5))) false false :!label _label_2)))
              (:`NewEnumerator1`
                (if (<= _returnvalue_y_5 (+ _returnvalue_y _returnvalue_2 -50.0))
                  (goto _label_2)))
              (:`NewEnumerator2`
                (if (>= _returnvalue_x_7 (- _returnvalue_x_3 _returnvalue_2 -50.0))
                  (goto _label_2)))
              (:`NewEnumerator3`
                (if (>= _returnvalue_y_5 (- _returnvalue_y _returnvalue_2 -50.0))
                  (goto _label_2))))))))))

(fn `SetPlayerBehaviour`
  (params (`Enter/Leave` :type Boolean)))

(fn `UserConstructionScript`
  (locals (`Z rotation` :type "Float (double-precision)"))
  (bind _box (`self.Box`))
  (bind _flowlength (`self.FlowLength`))
  (bind _niagara (`self.Niagara`))
  (bind _box_2 (`self.Box`))
  (bind _returnvalue (/ (`self.FlowLength`) 100.0))
  (bind (_relativescale3d_x _relativescale3d_y _relativescale3d_z) (`KismetMathLibrary.BreakVector` (`SceneComponent.RelativeScale3D` _box)))
  (bind (_relativelocation_x _relativelocation_y _relativelocation_z) (`KismetMathLibrary.BreakVector` (`SceneComponent.RelativeLocation` _box_2)))
  (`|ExecutionSequence`
    (:`then_0`
      (`SceneComponent.SetRelativeScale3D` _box (`KismetMathLibrary.MakeVector` (/ _flowlength 100.0) _relativescale3d_y _relativescale3d_z))
      (`SceneComponent.K2_SetRelativeLocation` _box_2 (`KismetMathLibrary.MakeVector` (/ _flowlength 2.0) _relativelocation_y _relativelocation_z) false false))
    (:`then_1`
      (switch `/Game/BlueprintClasses/Fans/FanOrientation` (`self.FanOrientation`)
        (:`NewEnumerator0`
          (set `local.Z rotation` 0.0)
          (set `self.MoveDirection` (1.0 0.0 0.0)))
        (:`NewEnumerator1`
          (set `local.Z rotation` 90.0)
          (set `self.MoveDirection` (0.0 1.0 0.0)))
        (:`NewEnumerator2`
          (set `local.Z rotation` 180.0)
          (set `self.MoveDirection` (-1.0 0.0 0.0)))
        (:`NewEnumerator3`
          (set `local.Z rotation` 270.0)
          (set `self.MoveDirection` (0.0 -1.0 0.0))))
      (`self.K2_SetActorRotation` (`KismetMathLibrary.MakeRotator` 0.0 0.0 (`local.Z rotation`))))
    (:`then_2`
      (`|ExecutionSequence`
        (:`then_0`
          (`FXSystemComponent.SetFloatParameter` _niagara "FountainLifetimeMin" (* _returnvalue 0.7)))
        (:`then_1`
          (`FXSystemComponent.SetFloatParameter` _niagara "FountainLifetimeMax" _returnvalue))))))