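; Switchable vertical fan that lifts the player and BP_OldBox crates up to a configurable flow height.
; The construction script fits the trigger box and Niagara lifetime to that height; overlaps track the player and boxes.
; While on, async physics tick raises them via SetActorLocation with gravity disabled, skipping grabbed boxes.
; Toggling swaps particles and core material; turning off restores gravity and wakes boxes so none hang mid-air.
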(event `self.ReceiveBeginPlay`
  (bind _base (`self.Base`))
  (bind _ns_quantumlift_blue (`self.NS_QuantumLift_Blue`))
  (`|ExecutionSequence`
    (:`then_0`
      (set `self.MoveRate` (/ (`self.HowManyUnitsPerSecond`) (`self.UpdatesPerSecond`)))
      (if (`self.IsOn`)
        ;[1 1 1] Animaiton
        (`FXSystemComponent.SetFloatParameter` _ns_quantumlift_blue "SpawnRate" 1.0 :!label _label)
        (`PrimitiveComponent.SetMaterial` _base 3 "/Game/BlenderFiles/Materials/Detector/OnCoreBlue.OnCoreBlue")
        (bind _returnvalue (`GameplayStatics.SpawnSoundAtLocation` (`self.Sound`) (`SceneComponent.K2_GetComponentLocation` (`self.Base`)) (struct) 1.0 1.0 0.0 "/Game/Audio/SoundAttenuationFan.SoundAttenuationFan" null))
        (bind _output_get (set `self.SpawnedSound` _returnvalue))
        (else
          (`FXSystemComponent.SetFloatParameter` _ns_quantumlift_blue "SpawnRate" 0.0 :!label _label_2)
          (`PrimitiveComponent.SetMaterial` _base 3 "/Game/BlenderFiles/Materials/Detector/OffCoreBlue.OffCoreBlue"))))
    (:`then_1`
      (`KismetSystemLibrary.DelayUntilNextTick`)
      (for _array_element (`PrimitiveComponent.GetOverlappingActors` (`self.Box`) "/Game/BlueprintClasses/BP_OldBox.BP_OldBox_C")
        (bind _asbp_old_box (cast `/Game/BlueprintClasses/BP_OldBox` _array_element))
        (if (`PrimitiveComponent.IsOverlappingComponent` (`self.Box`) (`/Game/BlueprintClasses/BP_OldBox.StaticMesh` _asbp_old_box))
          (`KismetArrayLibrary.Array_AddUnique` (`self.Boxes`) _asbp_old_box))))))

(event `/Game/BlueprintClasses/OnOffInterface.TurnOn`
  ;[1 1 1] Animaiton
  (set `self.IsOn` true)
  (`self.TurnedOn`)
  (goto _label))

(event `self.ReceiveAsyncPhysicsTick`
  (params (DeltaSeconds :type "Float (single-precision)") (SimSeconds :type "Float (single-precision)"))
  (if (`self.IsOn`)
    (`self.MoveObjectsIntoAir` DeltaSeconds)))

(event `/Game/BlueprintClasses/OnOffInterface.TurnOff`
  ;[1 1 1] Animaiton
  (set `self.IsOn` false)
  (`self.TurnedOff`)
  (goto _label_2))

(event `TurnedOn`
  (`self.SetPlayerBehaviour` true)
  (for _array_element (`self.Boxes`)
    (`self.SetBoxBehaviour` _array_element true)))

(event `TurnedOff`
  (`self.SetPlayerBehaviour` false)
  (for _array_element (`self.Boxes`)
    (`self.SetBoxBehaviour` _array_element)
    ;[1 1 1] Box Staying Mid Air Fix
    (`KismetSystemLibrary.Delay` (/ 1.0 (`self.UpdatesPerSecond`)))
    (`PrimitiveComponent.WakeRigidBody` (`/Game/BlueprintClasses/BP_OldBox.StaticMesh` _array_element) "None")))

(event `self.Box.OnComponentBeginOverlap`
  (params (OverlappedComponent :type "PrimitiveComponent Object Reference") (OtherActor :type "Actor Object Reference") (OtherComp :type "PrimitiveComponent Object Reference") (OtherBodyIndex :type Integer) (bFromSweep :type Boolean) (SweepResult :type "HitResult Structure (by ref)"))
  (bind _asbp_third_person_character (cast `/Game/ThirdPerson/Blueprints/BP_ThirdPersonCharacter` OtherActor)
    (:`then`
      (set `self.Player` _asbp_third_person_character))
    (:`CastFailed`
      (bind _asbp_old_box (cast `/Game/BlueprintClasses/BP_OldBox` OtherActor))
      (cast `StaticMeshComponent` OtherComp)
      (`KismetArrayLibrary.Array_AddUnique` (`self.Boxes`) _asbp_old_box))))

(event `self.Box.OnComponentEndOverlap`
  (params (OverlappedComponent :type "PrimitiveComponent Object Reference") (OtherActor :type "Actor Object Reference") (OtherComp :type "PrimitiveComponent Object Reference") (OtherBodyIndex :type Integer))
  (cast `/Game/ThirdPerson/Blueprints/BP_ThirdPersonCharacter` OtherActor
    (:`then`
      (`self.SetPlayerBehaviour` false)
      (set `self.Player` null))
    (:`CastFailed`
      (bind _asbp_old_box (cast `/Game/BlueprintClasses/BP_OldBox` OtherActor))
      (cast `StaticMeshComponent` OtherComp)
      (`self.SetBoxBehaviour` _asbp_old_box)
      (`KismetArrayLibrary.Array_RemoveItem` (`self.Boxes`) _asbp_old_box))))

(fn `MoveObjectsIntoAir`
  (params (DeltaTime :type "Float (double-precision)"))
  (locals (PlayerAlpha :type "Float (double-precision)"))
  (bind (_returnvalue_x _returnvalue_y _returnvalue_z) (`KismetMathLibrary.BreakVector` (`self.GetActorScale3D`)))
  (bind (_returnvalue_x_2 _returnvalue_y_2 _returnvalue_z_2) (`KismetMathLibrary.BreakVector` (`self.K2_GetActorLocation`)))
  (bind (_returnvalue_x_3 _returnvalue_y_3 _returnvalue_z_3) (`KismetMathLibrary.BreakVector` (`self.K2_GetActorLocation`)))
  (bind (_returnvalue_x_4 _returnvalue_y_4 _returnvalue_z_4) (`KismetMathLibrary.BreakVector` (`self.GetActorScale3D`)))
  (bind _player (`self.Player`))
  (bind (_returnvalue_x_5 _returnvalue_y_5 _returnvalue_z_5) (`KismetMathLibrary.BreakVector` (`self.K2_GetActorLocation` _player)))
  (bind _returnvalue (+ _returnvalue_z_3 (* (`self.FlowHight`) _returnvalue_z)))
  (set `self.MoveRate` (* DeltaTime (`self.HowManyUnitsPerSecond`)))
  (`|ExecutionSequence`
    (:`then_0`
      ;[1 1 1] Podnoszenie Gracza
      (if (`KismetSystemLibrary.IsValid` _player)
        (if (< _returnvalue_z_5 _returnvalue)
          (`self.SetPlayerBehaviour` true)
          (`self.K2_SetActorLocation` _player (`KismetMathLibrary.MakeVector` _returnvalue_x_5 _returnvalue_y_5 (+ _returnvalue_z_5 (`self.MoveRate`))) false false)
          (elif (and (> _returnvalue_z_5 _returnvalue) (`KismetArrayLibrary.Array_IsNotEmpty` (`self.Boxes`)))
            (`CharacterMovementComponent.AddForce` (`Character.CharacterMovement` _player) (0.0 0.0 100.0))))))
    (:`then_1`
      ;[1 1 1] Podnoszenie pudełek
      (for _array_element (`self.Boxes`)
        (if (`KismetSystemLibrary.IsValid` _array_element)
          (if (not (`/Game/BlueprintClasses/BP_OldBox.isBoxGrabbed?` _array_element))
            (bind (_returnvalue_x_6 _returnvalue_y_6 _returnvalue_z_6) (`KismetMathLibrary.BreakVector` (`self.K2_GetActorLocation` _array_element)))
            (if (< _returnvalue_z_6 (+ _returnvalue_z_2 (* (`self.FlowHight`) _returnvalue_z_4) -50.0))
              (`self.SetBoxBehaviour` _array_element true)
              (`self.K2_SetActorLocation` _array_element (`KismetMathLibrary.MakeVector` _returnvalue_x_6 _returnvalue_y_6 (+ _returnvalue_z_6 (`self.MoveRate`))) false false))))))))

(fn `SetBoxBehaviour`
  (params (Box :type "/Game/BlueprintClasses/BP_OldBox Object Reference") (`Enter/Leave` :type Boolean))
  (locals (StaticMesh :type "StaticMeshComponent Object Reference"))
  (bind _staticmesh (`local.StaticMesh`))
  (if (`KismetSystemLibrary.IsValid` Box)
    (set `local.StaticMesh` (`/Game/BlueprintClasses/BP_OldBox.StaticMesh` Box))
    (if `Enter/Leave`
      (if (`PrimitiveComponent.IsGravityEnabled` (`local.StaticMesh`))
        (`PrimitiveComponent.SetLinearDamping` _staticmesh 5.0)
        (`PrimitiveComponent.SetEnableGravity` _staticmesh false))
      (else
        (`PrimitiveComponent.SetLinearDamping` _staticmesh 0.01)
        (`PrimitiveComponent.SetEnableGravity` _staticmesh true)))))

(fn `SetPlayerBehaviour`
  (params (`Enter/Leave` :type Boolean))
  (locals (PlayerCharacterMovement :type "CharacterMovementComponent Object Reference"))
  (bind _playercharactermovement (`local.PlayerCharacterMovement`))
  (bind _player (`self.Player`))
  (if (`KismetSystemLibrary.IsValid` _player)
    (set `local.PlayerCharacterMovement` (`Character.CharacterMovement` _player))
    (if `Enter/Leave`
      (if (not (== (`CharacterMovementComponent.GravityScale` (`local.PlayerCharacterMovement`)) 0.0))
        (set `CharacterMovementComponent.GravityScale` 0.0 _playercharactermovement)
        (`MovementComponent.StopMovementImmediately` _playercharactermovement)
        (set `CharacterMovementComponent.BrakingDecelerationFalling` 1000.0 _playercharactermovement)
        (`CharacterMovementComponent.AddForce` _playercharactermovement (0.0 0.0 10.0)))
      (else
        (set `CharacterMovementComponent.GravityScale` 1.75 _playercharactermovement)
        (set `CharacterMovementComponent.BrakingDecelerationFalling` 0.0 _playercharactermovement)))))

(fn `UserConstructionScript`
  (bind _box (`self.Box`))
  (bind _flowhight (`self.FlowHight`))
  (bind _ns_quantumlift_blue (`self.NS_QuantumLift_Blue`))
  (bind _box_2 (`self.Box`))
  (bind _returnvalue (/ (`self.FlowHight`) 100.0))
  (bind (_relativescale3d_x _relativescale3d_y) (`KismetMathLibrary.BreakVector` (`SceneComponent.RelativeScale3D` _box)))
  (bind (_relativelocation_x _relativelocation_y) (`KismetMathLibrary.BreakVector` (`SceneComponent.RelativeLocation` _box_2)))
  (`|ExecutionSequence`
    (:`then_0`
      (`SceneComponent.SetRelativeScale3D` _box (`KismetMathLibrary.MakeVector` _relativescale3d_x _relativescale3d_y (/ _flowhight 100.0)))
      (`SceneComponent.K2_SetRelativeLocation` _box_2 (`KismetMathLibrary.MakeVector` _relativelocation_x _relativelocation_y (/ _flowhight 2.0)) false false))
    (:`then_1`
      (`|ExecutionSequence`
        (:`then_0`
          (`FXSystemComponent.SetFloatParameter` _ns_quantumlift_blue "FountainLifetimeMin" (* _returnvalue 0.7)))
        (:`then_1`
          (`FXSystemComponent.SetFloatParameter` _ns_quantumlift_blue "FountainLifetimeMax" _returnvalue))))))